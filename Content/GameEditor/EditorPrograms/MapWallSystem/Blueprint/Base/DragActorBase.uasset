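; Base actor for draggable items in the map wall editor, shown with collision only while the editor is in 2D mode.
; It binds to the game instance's 2D mode event and calls UpdateLocation on its create event.
; In 2D mode, Tick yaws the Box to the camera angle and measures a fixed span's screen and world size.
; Select, unselect and move events fire matching dispatchers, with selection tracked in DrIsSelect.
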(event `self.ReceiveBeginPlay`
  (add `/Game/GameEditor/EditorPrograms/Editor/EditorGameInstance.2DMode` (`/Game/GameEditor/EditorPrograms/Editor/FunctionLibrary/GetEditorGameInstance.GetEditorGameInstance`) (delegate `2DMode_事件_0`))
  (add `self.Create` (delegate `Create_事件_0`)))

(event `Create_事件_0`
  (`self.UpdateLocation`))

(event `2DMode_事件_0`
  (params (Is2D :type Boolean))
  (if Is2D
    (`self.SetActorHiddenInGame` false)
    (`self.SetActorEnableCollision` true)
    (else
      (`self.SetActorHiddenInGame` true)
      (`self.SetActorEnableCollision` false))))

(event `self.ReceiveTick`
  (params (DeltaSeconds :type "Float (single-precision)"))
  (bind _returnvalue (`self.K2_GetActorLocation`))
  (bind _returnvalue_2 (`GameplayStatics.GetPlayerController` 0))
  (bind _asmygame_editor_pawn (`/Game/GameEditor/EditorPrograms/Editor/FunctionLibrary/GetGamePawn.GetEditorPawn` 0))
  (bind _returnvalue_3 (+ _returnvalue (-10.0 0.0 0.0)))
  (bind _returnvalue_4 (+ _returnvalue (10.0 0.0 0.0)))
  (`/Engine/EditorBlueprintResources/StandardMacros.IsValid` _asmygame_editor_pawn
    (:`Is Valid`
      (if (`GameEditorPawn_Base.Enabled2DMode` _asmygame_editor_pawn)
        (`SceneComponent.K2_SetWorldRotation` (`self.Box`) (`KismetMathLibrary.MakeRotator` 0.0 0.0 (`.Angle` (`/Game/GameEditor/EditorPrograms/Editor/FunctionLibrary/BPFunctionLibrary.Get2DCameraRotation` 0))) false false)
        (set `self.2DSize` (`KismetMathLibrary.VSize2D` (- (`GameplayStatics.ProjectWorldToScreen` _returnvalue_2 _returnvalue_4) (`GameplayStatics.ProjectWorldToScreen` _returnvalue_2 _returnvalue_3))))
        (set `self.3DSize` (`KismetMathLibrary.VSize` (- _returnvalue_4 _returnvalue_3)))))))

(event `DR_Select`
  (set `self.Dr_IsSelect` true)
  (`self.DR_SelectEvent`))

(event `DR_UnSelect`
  (set `self.Dr_IsSelect` false)
  (`self.DR_UnSelectEvent`))

(event `MoveEvent`
  (`self.DR_MoveEvent`))

(fn `UserConstructionScript`)