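; WallPlaneUI is an actor in the map editor's wall system that draws a wall plane as a procedural mesh, with its screen-space widgets.
; Materials follow wall type, bearing status, delete state and level mode.
; Adding collision rebuilds the mesh and registers a delete-wall record in the GameInstance; Delete flags that record, removes enclosed hole widgets and destroys the actor.
; Tick pins the length-input widget to a projected world position.
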(event `self.ReceiveBeginPlay`
  (`|ExecutionSequence`
    (:`then_0`
      (bind _returnvalue (`|CreateWidget` "/Game/GameEditor/EditorPrograms/MapWallSystem/Widget/Comp/Aline.Aline_C"))
      (`UserWidget.AddToViewport` _returnvalue -10)
      (bind _output_get (set `self.Aline` _returnvalue))
      (set `/Game/GameEditor/EditorPrograms/MapWallSystem/Widget/Comp/Aline.WallPlaneUI` self _output_get))
    (:`then_1`
      (bind _returnvalue_2 (`|CreateWidget` "/Game/GameEditor/EditorPrograms/MapWallSystem/Widget/Comp/UserInputLengthWidget.UserInputLengthWidget_C"))
      (`CanvasPanel.AddChildToCanvas` (`/Game/GameEditor/EditorPrograms/MapWallSystem/Widget/W_WallDrawMainUI.Canvas_UserInputLength` (`/Game/GameEditor/EditorPrograms/MapWallSystem/Blueprint/FunctionLibrary/FunctionLibrary.GetWallMainWidget`)) _returnvalue_2)
      (bind _output_get_2 (set `self.InputRulerWidget` _returnvalue_2))
      (`Widget.SetVisibility` _output_get_2 "Hidden")
      (set `UserInputRulerWidget.bUseDisLengthFlag` false _returnvalue_2))))

(event `self.ReceiveDestroyed`
  (`Widget.RemoveFromParent` (`self.Aline`))
  (`Widget.RemoveFromParent` (`self.InputRulerWidget`)))

(event `self.Createplane`
  (bind _verlistpos (`self.VerListPos`))
  (bind _plane (`self.Plane`))
  (`ProceduralMeshComponent.CreateMeshSection_LinearColor` :`self` _plane :`Vertices` _verlistpos :`Triangles` (`self.TrianglesID`) :`Normals` (`self.NormalsDir`) :`UV0` (`/Game/GameEditor/EditorPrograms/Editor/FunctionLibrary/Geometry.VertexToUV` _verlistpos (100.0 100.0) (0.0 0.0) -90.0 false (`self.K2_GetActorLocation`) false (`KismetMathLibrary.GetVectorArrayAverage` _verlistpos)) :`bCreateCollision` (`self.bGeneratecollision`))
  (`PrimitiveComponent.SetMaterial` _plane 0 (`self.DefaultMaterialInstance`)))

(event `self.SetWallPlaneMaterial`
  (params (Type :type "EWallType Enum" :default "OriginalWall") (IsDelete :type Boolean) (IsBearingWall :type Boolean) (IsOpenNewWallType :type Boolean))
  (`|ExecutionSequence`
    (:`then_0`
      (if IsDelete
        (`PrimitiveComponent.SetMaterial` (`self.Plane`) 0 "/Game/GameEditor/EditorPrograms/MapWallSystem/Material/M_wall_Delete_Inst.M_wall_Delete_Inst")
        (set `self.DefaultMaterialInstance` "/Game/GameEditor/EditorPrograms/MapWallSystem/Material/M_wall_Delete_Inst.M_wall_Delete_Inst")
        (else
          (bind _returnvalue (`GameplayStatics.GetCurrentLevelName` true))
          (if (or (`KismetStringLibrary.EqualEqual_StrStr` _returnvalue "2DMode") IsOpenNewWallType)
            (if (`|EnumEquality` Type "NewWall")
              (if IsOpenNewWallType
                (`PrimitiveComponent.SetMaterial` (`self.Plane`) 0 "/Game/GameEditor/EditorPrograms/MapWallSystem/Material/M_wall_New_Inst.M_wall_New_Inst")
                (set `self.DefaultMaterialInstance` "/Game/GameEditor/EditorPrograms/MapWallSystem/Material/M_wall_New_Inst.M_wall_New_Inst")
                (else
                  (`PrimitiveComponent.SetMaterial` (`self.Plane`) 0 "/Game/GameEditor/EditorPrograms/MapWallSystem/Material/M_wall_New_Inst_New.M_wall_New_Inst_New")
                  (set `self.DefaultMaterialInstance` "/Game/GameEditor/EditorPrograms/MapWallSystem/Material/M_wall_New_Inst_New.M_wall_New_Inst_New")))
              (elif IsOpenNewWallType
                (if IsBearingWall
                  (`PrimitiveComponent.SetMaterial` (`self.Plane`) 0 "/Game/GameEditor/EditorPrograms/MapWallSystem/Material/BearingWallTexMaterial_Inst.BearingWallTexMaterial_Inst")
                  (set `self.DefaultMaterialInstance` "/Game/GameEditor/EditorPrograms/MapWallSystem/Material/BearingWallTexMaterial_Inst.BearingWallTexMaterial_Inst")
                  (else
                    (`PrimitiveComponent.SetMaterial` (`self.Plane`) 0 "/Game/GameEditor/EditorPrograms/MapWallSystem/Material/NoBearingWallTexMaterial_Inst.NoBearingWallTexMaterial_Inst")
                    (set `self.DefaultMaterialInstance` "/Game/GameEditor/EditorPrograms/MapWallSystem/Material/NoBearingWallTexMaterial_Inst.NoBearingWallTexMaterial_Inst")))
                (else
                  (if IsBearingWall :!label _label
                    (`PrimitiveComponent.SetMaterial` (`self.Plane`) 0 "/Game/GameEditor/EditorPrograms/MapWallSystem/Material/BearingWallMaterial.BearingWallMaterial")
                    (set `self.DefaultMaterialInstance` "/Game/GameEditor/EditorPrograms/MapWallSystem/Material/BearingWallMaterial_Inst.BearingWallMaterial_Inst")
                    (else
                      (`PrimitiveComponent.SetMaterial` (`self.Plane`) 0 "/Game/GameEditor/EditorPrograms/MapWallSystem/Material/NoBearingWallMaterial_Inst.NoBearingWallMaterial_Inst")
                      (set `self.DefaultMaterialInstance` "/Game/GameEditor/EditorPrograms/MapWallSystem/Material/NoBearingWallMaterial_Inst.NoBearingWallMaterial_Inst"))))))
            (else
              (goto _label))))))
    (:`then_1`
      (if IsOpenNewWallType
        _))))

(event `Addcollision`
  (bind _plane (`self.Plane`))
  (`/Engine/EditorBlueprintResources/StandardMacros.IsValid` (`self.Plane`)
    (:`Is Valid`
      (set `self.bGeneratecollision` true)
      (bind (_outposlist _planearea _height _startpos _endpos) (`self.CalculateSpot` (`self.VerListPos`)))
      (set `self.VerListPos` _outposlist)
      (`ProceduralMeshComponent.CreateMeshSection_LinearColor` :`self` _plane :`Vertices` _outposlist :`Triangles` (`self.TrianglesID`) :`Normals` (`self.NormalsDir`) :`UV0` (`/Game/GameEditor/EditorPrograms/Editor/FunctionLibrary/Geometry.VertexToUV` _outposlist (100.0 100.0) (0.0 0.0) -90.0 false (`self.K2_GetActorLocation`) false (`KismetMathLibrary.GetVectorArrayAverage` _outposlist)) :`bCreateCollision` (`self.bGeneratecollision`))
      (`PrimitiveComponent.SetMaterial` _plane 0 (`self.DefaultMaterialInstance`))
      (set `self.StructIndex` (`KismetArrayLibrary.Array_Length` (`CEditorGameInstance.DRDeleteWall` (`/Game/GameEditor/EditorPrograms/Editor/FunctionLibrary/GetEditorGameInstance.GetEditorGameInstance`))))
      (`KismetArrayLibrary.Array_Add` (`CEditorGameInstance.DRDeleteWall` (`/Game/GameEditor/EditorPrograms/Editor/FunctionLibrary/GetEditorGameInstance.GetEditorGameInstance`)) (make `DeleteWall` false _outposlist (/ (`KismetMathLibrary.GridSnap_Float` (/ _planearea 100.0) 1.0) 100.0) (`KismetMathLibrary.GridSnap_Float` (* (`self.Thickness`) 10.0) 1.0) _height _startpos _endpos (`self.ThicknessLeft`) (`self.ThicknessRight`)))
      (`self.SetDeleteWallText`))))

(event `self.Delete`
  (bind _structindex (`self.StructIndex`))
  (bind _drdeletewall (`CEditorGameInstance.DRDeleteWall` (`/Game/GameEditor/EditorPrograms/Editor/FunctionLibrary/GetEditorGameInstance.GetEditorGameInstance`)))
  (if (`KismetArrayLibrary.Array_IsValidIndex` _drdeletewall _structindex)
    (`|ExecutionSequence`
      (:`then_0`
        (bind _foundwidgets (`WidgetBlueprintLibrary.GetAllWidgetsOfClass` "/Game/GameEditor/EditorPrograms/MapWallSystem/Blueprint/Boolean_UMG.Boolean_UMG_C"))
        (for _array_element _foundwidgets
          (if (`|EnumEquality` (`BooleanBase.HolestatusType` _array_element) "EDRDeleteHole")
            (bind _returnvalue (`WallBuildSystem.JudgePointInPolygon` (`/Game/GameEditor/EditorPrograms/MapWallSystem/Blueprint/FunctionLibrary/FunctionLibrary.GetWallSystem` 0) (`self.VerListPos`) (`KismetMathLibrary.Conv_VectorToVector2D` (`.Loc` (break `DeleteHoleInfo` (`BooleanBase.DeleteHoleInfo` _array_element))))))
            (if _returnvalue
              (`Widget.RemoveFromParent` _array_element)))))
      (:`then_1`
        (bind _structout (setmembers `DeleteWall` :`StructRef` (`|GetArrayItem` _drdeletewall _structindex) :`isDelete` true))
        (`KismetArrayLibrary.Array_Set` _drdeletewall (`self.StructIndex`) _structout)
        (`self.K2_DestroyActor`)))))

(event `self.SetInputWidget`
  (params (LastCornerID :type Integer))
  (bind _inputrulerwidget (`self.InputRulerWidget`))
  (`/Engine/EditorBlueprintResources/StandardMacros.IsValid` _inputrulerwidget
    (:`Is Valid`
      (`Widget.SetVisibility` _inputrulerwidget "Visible")
      (bind _asuser_input_length_widget (cast `/Game/GameEditor/EditorPrograms/MapWallSystem/Widget/Comp/UserInputLengthWidget` _inputrulerwidget))
      (`Widget.SetKeyboardFocus` (`/Game/GameEditor/EditorPrograms/MapWallSystem/Widget/Comp/UserInputLengthWidget.SpinBox_0` _asuser_input_length_widget))
      (set `self.LastCornerID` LastCornerID))))

(event `self.ReceiveTick`
  (params (DeltaSeconds :type "Float (single-precision)"))
  (bind _inputrulerwidget (`self.InputRulerWidget`))
  (bind _screenlocation (`PlayerController.ProjectWorldLocationToScreen` (`GameplayStatics.GetPlayerController` 0) (`self.SpinBoxPos`) false))
  (`/Engine/EditorBlueprintResources/StandardMacros.IsValid` _inputrulerwidget
    (:`Is Valid`
      (if (`|EnumEquality` (`Widget.GetVisibility` _inputrulerwidget) "Visible")
        (`CanvasPanelSlot.SetPosition` (`WidgetLayoutLibrary.SlotAsCanvasSlot` (`Widget.GetParent` _inputrulerwidget)) (`KismetMathLibrary.MakeVector2D` (- (`KismetMathLibrary.BreakVector2D` _screenlocation) 30.0) (- (`.Y` (`KismetMathLibrary.BreakVector2D` _screenlocation)) 10.0)))))))

(event `self.AddDeleteWall`
  (`self.Addcollision`))

(fn `IsShowRuler`
  (returns (ReturnValue :type Boolean))
  (if (`/Game/GameEditor/EditorPrograms/Editor/EditorGameInstance.IsDrawingHouseMode` (`/Game/GameEditor/EditorPrograms/Editor/FunctionLibrary/GetEditorGameInstance.GetEditorGameInstance`))
    (if (`/Game/GameEditor/EditorPrograms/MapWallSystem/Blueprint/WallSystem.标尺` (`/Game/GameEditor/EditorPrograms/MapWallSystem/Blueprint/FunctionLibrary/FunctionLibrary.GetWallSystem` 0))
      (return true)
      (else
        _)))
  (return false))

(fn `PlanSetColor`
  (params (Isin :type Boolean))
  (`PrimitiveComponent.SetMaterial` (`self.Plane`) 0 (select `bool` Isin :`false` "/Game/GameEditor/EditorPrograms/MapWallSystem/Material/WallPlaneMaterial.WallPlaneMaterial" :`true` "/Game/_Basic/Materials/Materials_SecondLevel/M_wall2D.M_wall2D" :!type "MaterialInterface Object Reference")))

(fn `SetHiden`
  (params (Is :type Boolean))
  (bind _leftlabelwidget (`self.LeftLabelWidget`))
  (bind _rightlabelwidget (`self.RightLabelWidget`))
  (`|ExecutionSequence`
    (:`then_0`
      (`/Engine/EditorBlueprintResources/StandardMacros.IsValid` _leftlabelwidget
        (:`Is Valid`
          (`SceneComponent.SetVisibility` _leftlabelwidget Is false))))
    (:`then_1`
      (`/Engine/EditorBlueprintResources/StandardMacros.IsValid` _rightlabelwidget
        (:`Is Valid`
          (`SceneComponent.SetVisibility` _rightlabelwidget Is false))))))

(fn `UserConstructionScript`)