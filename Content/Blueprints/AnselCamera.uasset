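; Player camera manager that handles the end of NVIDIA Ansel photography sessions.
; When a session ends, it sets the ToAnselPicture flag on the game instance and calls QuitAnsel on the first Monitor actor in the level.
; The session start and multi-part capture events are empty.
; A helper, VerListToPoint2DList, flattens a vector list into 2D points by keeping X and Y, but nothing here calls it.
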(event `self.ReceiveBeginPlay`)

(event `self.OnPhotographyMultiPartCaptureStart`)

(event `self.OnPhotographySessionStart`)

(event `self.OnPhotographySessionEnd`
  (set `/Game/GameEditor/EditorPrograms/Editor/EditorGameInstance.ToAnselPicture` true (`/Game/GameEditor/EditorPrograms/Editor/FunctionLibrary/GetEditorGameInstance.GetEditorGameInstance`))
  (bind _outactors (`GameplayStatics.GetAllActorsOfClass` "/Game/GameEditor/EditorPrograms/Editor/Monitor.Monitor_C"))
  (`/Game/GameEditor/EditorPrograms/Editor/Monitor.QuitAnsel` (`|GetArrayItem` _outactors)))

(fn `UserConstructionScript`)

(fn `VerListToPoint2DList `
  (params (VList :type "Array of Vector Structure"))
  (returns (v2dlist :type "Array of Vector2D Structure"))
  (`KismetArrayLibrary.Array_Clear` (`self.vector2DList`))
  (for _array_element VList
    (`KismetArrayLibrary.Array_Add` (`self.vector2DList`) (`KismetMathLibrary.MakeVector2D` (.x _array_element) (.y _array_element))))
  (return (`self.vector2DList`)))