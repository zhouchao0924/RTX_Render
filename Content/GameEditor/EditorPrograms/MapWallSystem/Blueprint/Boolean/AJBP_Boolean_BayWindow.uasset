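; Bay window boolean (wall hole) actor for the house editor's wall system.
; Selection shows a Boolean_BayWindow attribute panel, in the main wall widget while drawing the house or in the pawn's attribute window otherwise.
; It builds a four-point cut section from its corner markers, accounting for the hole adapter's vertical flip.
; It also resets its materials to wall-config defaults and nudges the selected face's UV offset through the panel.
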(event `self.ReceiveBeginPlay`
  (`parent.ReceiveBeginPlay`)
  (add `self.OnSelect` (delegate `OnSelect_Event`)))

(event `OnSelect_Event` :!signature `self.OnSelect`
  (params (isSelect :type Boolean))
  (bind _booleanbaywindow (`self.BooleanBayWindow`))
  (if (`/Game/GameEditor/EditorPrograms/Editor/EditorGameInstance.IsDrawingHouseMode` (`/Game/GameEditor/EditorPrograms/Editor/FunctionLibrary/GetEditorGameInstance.GetEditorGameInstance`))
    (if isSelect
      (`/Engine/EditorBlueprintResources/StandardMacros.IsValid` (`self.BooleanBayWindow`)
        (:`Is Valid`
          _)
        (:`Is Not Valid`
          (bind _returnvalue (`|CreateWidget` "/Game/GameEditor/EditorPrograms/MapWallSystem/Widget/Boolean/Boolean_BayWindow.Boolean_BayWindow_C" null self))
          (set `self.BooleanBayWindow` _returnvalue)))
      (`/Game/GameEditor/EditorPrograms/MapWallSystem/Widget/W_WallDrawMainUI.AddAttributes` (`/Game/GameEditor/EditorPrograms/MapWallSystem/Blueprint/FunctionLibrary/FunctionLibrary.GetWallMainWidget`) (`self.BooleanBayWindow`))
      (else
        (`/Engine/EditorBlueprintResources/StandardMacros.IsValid` _booleanbaywindow
          (:`Is Valid`
            (`Widget.RemoveFromParent` _booleanbaywindow)))))
    (else
      (`self.ShowAttributesIn3D` isSelect))))

(event `self.ClearMaterial`
  (bind (_roomclass _craft) (`/Game/GameEditor/EditorPrograms/MapWallSystem/Blueprint/FunctionLibrary/FunctionLibrary.GetDefaultRoomClassAndCraft` (`DROperationHouseFunctionLibrary.GetConfigModelIDByType` "EDRWallConfig")))
  (for _index (range 4)
    (`self.SetMaterial` _index null (`DROperationHouseFunctionLibrary.GetConfigModelIDByType` "EDRWallConfig") true null _roomclass (`|MakeArray` _craft))))

(fn `AddUVOffset`
  (params (Delt :type "Float (double-precision)") (UorV :type Boolean))
  (returns (Ret :type Boolean))
  (locals (Local_UorV :type Boolean) (Local_Delt :type "Float (double-precision)") (Local_UV :type "DRUV Structure") (Local_HoleUVs :type "Array of DRUV Structure"))
  (bind _local_delt (`local.Local_Delt`))
  (bind ((`UVOffset` _uvoffset)) (break `DRUV` (`local.Local_UV`)))
  (set `local.Local_Delt` Delt)
  (set `local.Local_UorV` UorV)
  (bind _returnvalue (`DRProjData.GetAdapter` (`DRProjData.GetProjectDataManager`) (`self.ObjectID`)))
  (bind _asdrwindow_hole_adapter (cast `DRWindowHoleAdapter` _returnvalue))
  (set `local.Local_HoleUVs` (`DRHoleAdapter.GetHoleUVs` _asdrwindow_hole_adapter))
  (`/Engine/EditorBlueprintResources/StandardMacros.IsValid` (`self.DoorAttributes`)
    (:`Is Valid`
      (bind _asboolean_bay_window (cast `/Game/GameEditor/EditorPrograms/MapWallSystem/Widget/Boolean/Boolean_BayWindow` (`self.DoorAttributes`))
        (:`then`
          (set `local.Local_UV` (`|GetArrayItem` (`local.Local_HoleUVs`) (`/Game/GameEditor/EditorPrograms/MapWallSystem/Widget/Boolean/Boolean_BayWindow.SelectIndex` _asboolean_bay_window)))
          (`/Game/GameEditor/EditorPrograms/MapWallSystem/Widget/C_Vector2D.SetValue` (`/Game/GameEditor/EditorPrograms/MapWallSystem/Widget/Boolean/Boolean_BayWindow.UVOffset` _asboolean_bay_window) (select `bool` (`local.Local_UorV`) :`false` (+ _uvoffset (`KismetMathLibrary.MakeVector2D` 0.0 _local_delt)) :`true` (+ _uvoffset (`KismetMathLibrary.MakeVector2D` _local_delt))))
          (return true))
        (:`CastFailed`
          _)))
    (:`Is Not Valid`
      _))
  (return false))

(fn `GetBooleanSection`
  (returns (Vertices :type "Array of Vector Structure"))
  (locals (Local_Vertical :type Boolean :default false))
  (bind _returnvalue (`self.K2_GetActorLocation`))
  (bind _yaw (.yaw (`self.K2_GetActorRotation`)))
  (bind _returnvalue_2 (+ (.z (`SceneComponent.RelativeLocation` (`self.LitUp`))) 10.0))
  (bind _returnvalue_3 (+ (`KismetSystemLibrary.MakeLiteralDouble` (`self.Length`)) (`KismetMathLibrary.VSize` (- (`SceneComponent.K2_GetComponentLocation` (`self.L_P1`)) (`SceneComponent.K2_GetComponentLocation` (`self.L_P2`))))))
  (bind _returnvalue_4 (`KismetMathLibrary.Conv_RotatorToVector` (`KismetMathLibrary.MakeRotator` (.roll (`self.K2_GetActorRotation`)) (.pitch (`self.K2_GetActorRotation`)) (select `bool` (`local.Local_Vertical`) :`false` _yaw :`true` (- _yaw 180.0)))))
  (bind _returnvalue_5 (`DRProjData.GetAdapter` (`DRProjData.GetProjectDataManager`) (`self.ObjectID`)))
  (bind _asdrhole_adapter (cast `DRHoleAdapter` _returnvalue_5))
  (set `local.Local_Vertical` (`DRHoleAdapter.GetVerticalFlip` _asdrhole_adapter))
  (return (`|MakeArray` (`KismetMathLibrary.MakeVector` (.x (- (+ (`SceneComponent.K2_GetComponentLocation` (`self.L_P2`)) (* _returnvalue_4 _returnvalue_3)) _returnvalue)) (.y (- (+ (`SceneComponent.K2_GetComponentLocation` (`self.L_P2`)) (* _returnvalue_4 _returnvalue_3)) _returnvalue)) _returnvalue_2) (`KismetMathLibrary.MakeVector` (.x (- (+ (`SceneComponent.K2_GetComponentLocation` (`self.R_P2`)) (* _returnvalue_4 _returnvalue_3)) _returnvalue)) (.y (- (+ (`SceneComponent.K2_GetComponentLocation` (`self.R_P2`)) (* _returnvalue_4 _returnvalue_3)) _returnvalue)) _returnvalue_2) (`KismetMathLibrary.MakeVector` (.x (- (`SceneComponent.K2_GetComponentLocation` (`self.R_P2`)) _returnvalue)) (.y (- (`SceneComponent.K2_GetComponentLocation` (`self.R_P2`)) _returnvalue)) _returnvalue_2) (`KismetMathLibrary.MakeVector` (.x (- (`SceneComponent.K2_GetComponentLocation` (`self.L_P2`)) _returnvalue)) (.y (- (`SceneComponent.K2_GetComponentLocation` (`self.L_P2`)) _returnvalue)) _returnvalue_2))))

(fn `ShowAttributesIn3D`
  (params (`Select?` :type Boolean))
  (bind _windowattribute (`self.WindowAttribute`))
  (if `Select?`
    (`/Engine/EditorBlueprintResources/StandardMacros.IsValid` (`self.WindowAttribute`)
      (:`Is Valid`
        (cast `/Game/GameEditor/EditorPrograms/MapWallSystem/Widget/Boolean/Boolean_BayWindow` (`self.WindowAttribute`)))
      (:`Is Not Valid`
        (bind _returnvalue (`/Game/GameEditor/EditorPrograms/Widget/C_AttributeWindow.AddAttribute` (`/Game/GameEditor/EditorPrograms/Editor/MyGameEditorPawn.AttributeWindow` (`/Game/GameEditor/EditorPrograms/Editor/FunctionLibrary/GetGamePawn.GetEditorPawn` 0)) "/Game/GameEditor/EditorPrograms/MapWallSystem/Widget/Boolean/Boolean_BayWindow.Boolean_BayWindow_C"))
        (bind _output_get (set `self.WindowAttribute` _returnvalue))
        (bind _asboolean_bay_window (cast `/Game/GameEditor/EditorPrograms/MapWallSystem/Widget/Boolean/Boolean_BayWindow` _output_get))
        (set `/Game/GameEditor/EditorPrograms/MapWallSystem/Widget/Boolean/Boolean_BayWindow.Boolean` self _asboolean_bay_window)
        (`/Game/GameEditor/EditorPrograms/MapWallSystem/Widget/Boolean/Boolean_BayWindow.SetSizeBoxVisible` _asboolean_bay_window false)))
    (else
      (`/Engine/EditorBlueprintResources/StandardMacros.IsValid` _windowattribute
        (:`Is Valid`
          (`Widget.RemoveFromParent` _windowattribute)
          (set `self.WindowAttribute` null))))))

(fn `UserConstructionScript`
  (`parent.UserConstructionScript`))