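; Actor in the map editor's wall system that displays a raised copy of a boolean object's Under mesh.
; On BeginPlay, if MBoolean's Under mesh is valid, it reads procedural mesh section 0 and offsets the vertices vertically by Z through MoveUpDx.
; It builds the Plane procedural mesh from those vertices with the original triangles and normals, then applies the default wall material.
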(event `self.ReceiveBeginPlay`
  (bind _plane (`self.Plane`))
  (bind _under (`Wall_Boolean_Base.Under` (`self.M_Boolean`)))
  (`/Engine/EditorBlueprintResources/StandardMacros.IsValid` _under
    (:`Is Valid`
      (bind _returnvalue (`ProcMeshFunctionLibrary.GetProcMeshSection` _under))
      (bind (_vertices _triangles _normals) (break `ProcMeshConfig` _returnvalue))
      (bind _out (`self.MoveUpDx` _vertices (`self.z`)))
      (`ProceduralMeshComponent.CreateMeshSection_LinearColor` :`self` _plane :`Vertices` _out :`Triangles` _triangles :`Normals` _normals)
      (`PrimitiveComponent.SetMaterial` _plane 0 "/Game/GameEditor/EditorPrograms/MapWallSystem/Material/DefaultWallMaterial_Inst.DefaultWallMaterial_Inst"))))

(fn `MoveUpDx`
  (params (in :type "Array of Vector Structure") (dx :type "Float (double-precision)"))
  (returns (out :type "Array of Vector Structure"))
  (locals (temparr :type "Array of Vector Structure"))
  (for _array_element in
    (`KismetArrayLibrary.Array_Add` (`local.temparr`) (+ _array_element (`KismetMathLibrary.MakeVector` 0.0 0.0 dx))))
  (return (`local.temparr`)))

(fn `UserConstructionScript`)