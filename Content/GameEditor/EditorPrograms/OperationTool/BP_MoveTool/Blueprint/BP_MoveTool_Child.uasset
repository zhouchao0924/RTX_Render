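; Move gizmo for the in-game editor, extending a parent move tool to drag the selected actors.
; Tick applies grid size, 2D-mode handles and guide-line visibility, then positions the gizmo, with cursor-trace surface snapping or a polygon limit for ceiling mouldings.
; Parent tool events drive pawn state, cursor and product widget updates; closing a move saves attached actors' locations and notifies cabinets.
; SetLabelVisible and the area-switching functions are stubbed out.
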(event `self.ReceiveTick`
  (params (DeltaSeconds :type "Float (single-precision)"))
  (bind (_location _bblockinghit) (`self.LineTrace`))
  (bind (_location_2 _bblockinghit_2) (`self.LineTrace`))
  (bind _movelocation (`self.MoveLocation`))
  (bind _movelocation_2 (`self.MoveLocation`))
  (bind _yz (`self.YZ`))
  (bind (_returnvalue_x _returnvalue_y _returnvalue_z) (`KismetMathLibrary.BreakVector` (`SceneComponent.K2_GetComponentScale` (`self.ScaleRoot`))))
  (bind _output (`|GetArrayItem` (`/Game/GameEditor/EditorPrograms/Editor/EditorBaseFunctionController.Actorlist` (`/Game/GameEditor/EditorPrograms/Editor/MyGameEditorPawn.EditorFunction` (`/Game/GameEditor/EditorPrograms/Editor/FunctionLibrary/GetGamePawn.GetEditorPawn` 0)))))
  (bind _staticmesh (`/Game/GameEditor/EditorPrograms/MapObjectSystem/Base/MapBase.StaticMesh` (cast `/Game/GameEditor/EditorPrograms/MapObjectSystem/Base/MapBase_Object` (`|GetArrayItem` (`/Game/GameEditor/EditorPrograms/Editor/EditorBaseFunctionController.Actorlist` (`/Game/GameEditor/EditorPrograms/Editor/MyGameEditorPawn.EditorFunction` (`/Game/GameEditor/EditorPrograms/Editor/FunctionLibrary/GetGamePawn.GetEditorPawn` 0)))) :!pure true)))
  (bind (_origin _boxextent) (`KismetSystemLibrary.GetComponentBounds` _staticmesh))
  (set `self.GridSize` (`KismetMathLibrary.Conv_IntToDouble` (`GameEditorPawn_Base.LocationAlignmentValue` (`/Game/GameEditor/EditorPrograms/Editor/FunctionLibrary/GetGamePawn.GetEditorPawn` 0))))
  (`|ExecutionSequence`
    (:`then_0`
      (set `self.2DMode` (`GameEditorPawn_Base.Enabled2DMode` (`/Game/GameEditor/EditorPrograms/Editor/FunctionLibrary/GetGamePawn.GetEditorPawn` 0)))
      (set `self.2DSize` (/ (`CameraComponent.OrthoWidth` (`/Game/GameEditor/EditorPrograms/Editor/MyGameEditorPawn.2DCamera` (`/Game/GameEditor/EditorPrograms/Editor/FunctionLibrary/GetGamePawn.GetEditorPawn` 0))) 1300.0))
      (`parent.ReceiveTick` 0.0)
      (`|ExecutionSequence`
        (:`then_0`
          (if (`GameEditorPawn_Base.Enabled2DMode` (`/Game/GameEditor/EditorPrograms/Editor/FunctionLibrary/GetGamePawn.GetEditorPawn` 0))
            (`SceneComponent.SetVisibility` _yz false false)
            (`SceneComponent.SetVisibility` (`self.Z`) false false)
            (`SceneComponent.SetVisibility` (`self.XZ`) false false)
            (`PrimitiveComponent.SetCollisionEnabled` _yz "NoCollision")
            (`PrimitiveComponent.SetCollisionEnabled` (`self.XZ`) "NoCollision")
            (`PrimitiveComponent.SetCollisionEnabled` (`self.Z`) "NoCollision")
            (else
              (`SceneComponent.SetVisibility` (`self.Z`) true false)
              (`SceneComponent.SetVisibility` (`self.XZ`) true false)
              (`SceneComponent.SetVisibility` _yz true false)
              (`PrimitiveComponent.SetCollisionEnabled` _yz "QueryAndPhysics")
              (`PrimitiveComponent.SetCollisionEnabled` (`self.XZ`) "QueryAndPhysics")
              (`PrimitiveComponent.SetCollisionEnabled` (`self.Z`) "QueryAndPhysics"))))
        (:`then_1`
          (set `self.H` (`KismetMathLibrary.FClamp` _returnvalue_z 0.0 5.0))
          (if (not (`self.Temp_StartMove`))
            (if (`GameEditorPawn_Base.AuxiliaryLine` (`/Game/GameEditor/EditorPrograms/Editor/FunctionLibrary/GetGamePawn.GetEditorPawn` 0)) :!label _label
              (if (`.OpenCtrlOperating_92_46FC354E4CD3AB92DEB4D296CD0FE4B8` (break `/Game/GameEditor/EditorPrograms/Editor/Structure/EditorConfig` (`/Game/GameEditor/EditorPrograms/Editor/EditorGameInstance.EditorConfig` (`/Game/GameEditor/EditorPrograms/Editor/FunctionLibrary/GetEditorGameInstance.GetEditorGameInstance`)))) :!label _label_2
                (`SceneComponent.SetVisibility` (`self.DR_Z`) true false)
                (`SceneComponent.SetVisibility` (`self.DR_Y`) true false)
                (`SceneComponent.SetVisibility` (`self.DR_X`) true false)
                (else
                  (`SceneComponent.SetVisibility` (`self.DR_Z`) false false :!label _label_3)
                  (`SceneComponent.SetVisibility` (`self.DR_Y`) false false)
                  (`SceneComponent.SetVisibility` (`self.DR_X`) false false)))
              (elif (`PeExtendedToolKitBPLibrary.IsCtrlClick`)
                (if (`GameEditorPawn_Base.GeometryMode` (`/Game/GameEditor/EditorPrograms/Editor/FunctionLibrary/GetGamePawn.GetEditorPawn` 0))
                  (goto _label_3)
                  (else
                    (goto _label_2)))
                (else
                  (goto _label_3))))
            (elif (`GameEditorPawn_Base.SurfaceCapture` (`/Game/GameEditor/EditorPrograms/Editor/FunctionLibrary/GetGamePawn.GetEditorPawn` 0))
              (if (`.bSuccess` (cast `/Game/GameEditor/EditorPrograms/Editor/SlicerBlueprint` _output :!pure true))
                (set `self.Loc` (select `bool` (== (`self.HitComp`) (`self.XYZ`)) :`false` _movelocation_2 :`true` (select `bool` _bblockinghit :`false` _movelocation_2 :`true` _location)))
                (`self.K2_SetActorLocation` (- (`self.Loc`) (`self.AlignmentOffset`)) :!label _label_4)
                (goto _label)
                (elif (`KismetArrayLibrary.Array_IsValidIndex` (`/Game/GameEditor/EditorPrograms/Editor/EditorBaseFunctionController.Actorlist` (`/Game/GameEditor/EditorPrograms/Editor/MyGameEditorPawn.EditorFunction` (`/Game/GameEditor/EditorPrograms/Editor/FunctionLibrary/GetGamePawn.GetEditorPawn` 0))))
                  (set `self.Loc` (select `bool` (== (`self.HitComp`) (`self.XYZ`)) :`false` _movelocation :`true` (select `bool` _bblockinghit_2 :`false` _movelocation :`true` (+ _location_2 (`KismetMathLibrary.MakeVector` 0.0 0.0 (.z (+ _boxextent (- (`SceneComponent.K2_GetComponentLocation` _staticmesh) _origin))))))))
                  (goto _label_4)))
              (else
                (bind _ascustom_moulding_ceil (cast `/Game/GameEditor/EditorPrograms/MapObjectSystem/S_CustomModel/CustomMouldingCeil` _output)
                  (:`then`
                    (bind _returnvalue (`RoomActor.isPointInPolygons2D` (`.Points` (break `MouldingCeilingInfo` (`/Game/GameEditor/EditorPrograms/MapObjectSystem/S_CustomModel/CustomMouldingCeil.MouldingCeilingInfo` _ascustom_moulding_ceil))) (`KismetMathLibrary.Conv_VectorToVector2D` (`self.MoveLocation`)) 1000.0))
                    (if _returnvalue
                      (set `self.Loc` (`self.MoveLocation`) :!label _label_5)
                      (goto _label_4)))
                  (:`CastFailed`
                    (goto _label_5)))))))))
    (:`then_1`
      (if (`GameEditorPawn_Base.WorldMode` (`/Game/GameEditor/EditorPrograms/Editor/FunctionLibrary/GetGamePawn.GetEditorPawn` 0))
        (`SceneComponent.K2_SetWorldRotation` :`self` (`self.ScaleRoot`))))))

(event `self.ReceiveBeginPlay`
  (add `self.OnMove` (delegate `OnMove_事件_0`))
  (`/Game/GameEditor/EditorPrograms/Editor/EditorGameInstance.ToolBeginPlay` (`/Game/GameEditor/EditorPrograms/Editor/FunctionLibrary/GetEditorGameInstance.GetEditorGameInstance`))
  (set `self.2DSize` (/ (`CameraComponent.OrthoWidth` (`/Game/GameEditor/EditorPrograms/Editor/MyGameEditorPawn.2DCamera` (`/Game/GameEditor/EditorPrograms/Editor/FunctionLibrary/GetGamePawn.GetEditorPawn` 0))) 1300.0))
  (set `self.2DMode` (`GameEditorPawn_Base.Enabled2DMode` (`/Game/GameEditor/EditorPrograms/Editor/FunctionLibrary/GetGamePawn.GetEditorPawn` 0)))
  (set `self.MoveLocation` (`self.K2_GetActorLocation`))
  (`parent.ReceiveBeginPlay`)
  (add `self.ActivateMouse` (delegate `ActivateMouse_Event`))
  (add `self.ReleaseTheMouse` (delegate `ReleaseTheMouse_Event`))
  (add `self.ActivateMove` (delegate `ActivateMove_Event`))
  (add `self.CloseMove` (delegate `CloseMove_Event`)))

(event `self.ReceiveDestroyed`
  (bind _returnvalue (`GameplayStatics.GetPlayerController` 0))
  (bind _asmygame_editor_pawn (`/Game/GameEditor/EditorPrograms/Editor/FunctionLibrary/GetGamePawn.GetEditorPawn` 0))
  (bind _cursorumg (`/Game/GameEditor/EditorPrograms/Editor/EditorGameInstance.CursorUMG` (`/Game/GameEditor/EditorPrograms/Editor/FunctionLibrary/GetEditorGameInstance.GetEditorGameInstance`)))
  (`parent.ReceiveDestroyed`)
  (`/Engine/EditorBlueprintResources/StandardMacros.IsValid` _asmygame_editor_pawn :!label _label_6
    (:`Is Valid`
      (set `GameEditorPawn_Base.Move` false _asmygame_editor_pawn))
    (:`Is Not Valid`
      _))
  (`/Engine/EditorBlueprintResources/StandardMacros.IsValid` _returnvalue
    (:`Is Valid`
      (set `PlayerController.CurrentMouseCursor` "Default" _returnvalue)
      (`/Engine/EditorBlueprintResources/StandardMacros.IsValid` _cursorumg
        (:`Is Valid`
          (`/Game/GameEditor/EditorPrograms/Widget/Comp/C_Cursor.SetCursorMode` _cursorumg 0))))))

(event `ActivateMove_Event`
  (bind _cursorumg (`/Game/GameEditor/EditorPrograms/Editor/EditorGameInstance.CursorUMG` (`/Game/GameEditor/EditorPrograms/Editor/FunctionLibrary/GetEditorGameInstance.GetEditorGameInstance`)))
  (`self.SetLabelVisible` false)
  (set `GameEditorPawn_Base.Move` true (`/Game/GameEditor/EditorPrograms/Editor/FunctionLibrary/GetGamePawn.GetEditorPawn` 0))
  (`/Engine/EditorBlueprintResources/StandardMacros.IsValid` _cursorumg
    (:`Is Valid`
      (`/Game/GameEditor/EditorPrograms/Widget/Comp/C_Cursor.SetCursorMode` _cursorumg 1))))

(event `CloseMove_Event`
  (bind _actor (`self.GetCabinetActor`))
  (`/Engine/EditorBlueprintResources/StandardMacros.IsValid` _actor
    (:`Is Valid`
      (`/Game/GameEditor/EditorPrograms/Editor/MyGameEditorPawn.NotifyCabinetTransform` (`/Game/GameEditor/EditorPrograms/Editor/FunctionLibrary/GetGamePawn.GetEditorPawn` 0) _actor))
    (:`Is Not Valid`
      _))
  (`self.SetLabelVisible` true)
  (`self.SaveMovedActorLocation`)
  (`/Game/GameEditor/EditorPrograms/Editor/EditorGameInstance.MoveToolS` (`/Game/GameEditor/EditorPrograms/Editor/FunctionLibrary/GetEditorGameInstance.GetEditorGameInstance`))
  (goto _label_6))

(event `ActivateMouse_Event`
  (bind _cursorumg (`/Game/GameEditor/EditorPrograms/Editor/EditorGameInstance.CursorUMG` (`/Game/GameEditor/EditorPrograms/Editor/FunctionLibrary/GetEditorGameInstance.GetEditorGameInstance`)))
  (set `GameEditorPawn_Base.IsMoving` true (`/Game/GameEditor/EditorPrograms/Editor/FunctionLibrary/GetGamePawn.GetEditorPawn` 0))
  (`|ExecutionSequence`
    (:`then_0`
      (set `self.AlignmentOffset` (- (`self.K2_GetActorLocation`) (`self.K2_GetActorLocation`))))
    (:`then_1`
      (`/Engine/EditorBlueprintResources/StandardMacros.IsValid` _cursorumg
        (:`Is Valid`
          (`/Game/GameEditor/EditorPrograms/Widget/Comp/C_Cursor.SetCursorMode` _cursorumg 2))))))

(event `OnMove_事件_0`
  (`/Game/GameEditor/EditorPrograms/Editor/EditorGameInstance.MoveToolUpDate` (`/Game/GameEditor/EditorPrograms/Editor/FunctionLibrary/GetEditorGameInstance.GetEditorGameInstance`))
  (`self.ConfirmCustomProductLocation`))

(event `ReleaseTheMouse_Event`
  (bind _cursorumg (`/Game/GameEditor/EditorPrograms/Editor/EditorGameInstance.CursorUMG` (`/Game/GameEditor/EditorPrograms/Editor/FunctionLibrary/GetEditorGameInstance.GetEditorGameInstance`)))
  (set `GameEditorPawn_Base.IsMoving` false (`/Game/GameEditor/EditorPrograms/Editor/FunctionLibrary/GetGamePawn.GetEditorPawn` 0))
  (`/Engine/EditorBlueprintResources/StandardMacros.IsValid` _cursorumg
    (:`Is Valid`
      (`/Game/GameEditor/EditorPrograms/Widget/Comp/C_Cursor.SetCursorMode` _cursorumg 0))))

(fn `ChagneToArea`)

(fn `ChangeAreaOrNoArea`
  (locals (Local_Actor :type "/Game/GameEditor/EditorPrograms/MapObjectSystem/Base/MapBase_Object Object Reference")))

(fn `ChangeToNoArea`)

(fn `CheckChildActorIsDoorOrWindow`
  (returns (IsDoorAndWindow :type Boolean))
  (for _array_element (`self.GetAttachedActors`)
    (bind _asmap_base_object (cast `/Game/GameEditor/EditorPrograms/MapObjectSystem/Base/MapBase_Object` _array_element)
      (:`then`
        (if (not (`/Game/GameEditor/EditorPrograms/MapObjectSystem/Base/MapBase_Object.IsDoorAndWindow` _asmap_base_object))
          (return false)))
      (:`CastFailed`
        (return false))))
  (return true))

(fn `ConfirmCustomProductLocation`
  (locals (LocalCustomProductFactorty :type "/Game/UMG/CustomProductFactory/CustomProductFactory_WD Object Reference") (LocalAttachedList :type "Array of Actor Object Reference"))
  (bind (_widget _return) (`/Game/GameEditor/EditorPrograms/MapWallSystem/Blueprint/FunctionLibrary/FunctionLibrary.IsInCustomProductInfoTable`))
  (set `local.LocalCustomProductFactorty` _widget)
  (if _return
    (set `local.LocalAttachedList` (`self.GetAttachedActors`))
    (if (and (== (`KismetArrayLibrary.Array_Length` (`local.LocalAttachedList`)) 1) (`/Game/GameEditor/EditorPrograms/MapWallSystem/Blueprint/FunctionLibrary/FunctionLibrary.==` (`|GetArrayItem` (`local.LocalAttachedList`)) (`/Game/UMG/CustomProductFactory/CustomProductFactory_WD.TargetActor_Ref` (`local.LocalCustomProductFactorty`))))
      (`/Game/UMG/CustomProductFactory/CustomProductFactory_WD.ChangeWidgetLocation` (`local.LocalCustomProductFactorty`) (`self.K2_GetActorLocation`)))))

(fn `DrawLine`
  (params (InRot :type "Rotator Structure") (LineColor :type "LinearColor Structure") (Text :type String) (TextRot :type "Rotator Structure") (TextLocation :type "Vector Structure"))
  (bind _h (`self.H`))
  (bind _returnvalue (* (`KismetMathLibrary.Conv_RotatorToVector` InRot) 9999999.0))
  (bind _returnvalue_2 (`SceneComponent.K2_GetComponentLocation` (`self.Root`)))
  ;[1 1 1] X
  (`KismetSystemLibrary.DrawDebugString` TextLocation Text null)
  (`KismetSystemLibrary.DrawDebugLine` _returnvalue_2 (+ _returnvalue_2 _returnvalue) LineColor 0.0 _h)
  (`KismetSystemLibrary.DrawDebugLine` _returnvalue_2 (* _returnvalue -1.0) LineColor 0.0 _h)
  (return))

(fn `GetCabinetActor`
  (returns (actor :type "Actor Object Reference"))
  (bind _output (`|GetArrayItem` (`self.GetAttachedActors`)))
  (bind _asfur_actor (cast `/Game/UMG/CreateWidget/FurActor` _output)
    (:`then`
      (return _asfur_actor))
    (:`CastFailed`
      (bind _assku_component_actor (cast `SkuComponentActor` _output)
        (:`then`
          (return _assku_component_actor))
        (:`CastFailed`
          (return null))))))

(fn `LineTrace`
  (returns (Location :type "Vector Structure") (bBlockingHit :type Boolean))
  (bind (_worldlocation _worlddirection) (`PlayerController.DeprojectMousePositionToWorld` (`GameplayStatics.GetPlayerController` 0)))
  (bind _outhit (`KismetSystemLibrary.LineTraceSingleForObjects` _worldlocation (+ _worldlocation (* _worlddirection 10000000.0)) (`|MakeArray` "ObjectTypeQuery1" :!type "EObjectTypeQuery Enum") true (`/Game/GameEditor/EditorPrograms/Editor/EditorBaseFunctionController.Actorlist` (`/Game/GameEditor/EditorPrograms/Editor/MyGameEditorPawn.EditorFunction` (`/Game/GameEditor/EditorPrograms/Editor/FunctionLibrary/GetGamePawn.GetEditorPawn` 0)))))
  (bind (_bblockinghit _binitialoverlap _time _distance _location) (`GameplayStatics.BreakHitResult` _outhit))
  (return _location _bblockinghit))

(fn `SaveMovedActorLocation`
  (for _array_element (`self.GetAttachedActors`)
    (bind _asmap_base_object (cast `/Game/GameEditor/EditorPrograms/MapObjectSystem/Base/MapBase_Object` _array_element)
      (:`then`
        (`/Game/GameEditor/EditorPrograms/MapObjectSystem/Base/MapBase_Object.UpdateLocation` _asmap_base_object))
      (:`CastFailed`
        (bind _asgroup_actor_bp (cast `/Game/GameEditor/EditorPrograms/Editor/GroupActor_BP` _array_element))
        (for _array_element_2 (`GroupActorBase.GroupActors` _asgroup_actor_bp)
          (bind _asmap_base_object_2 (cast `/Game/GameEditor/EditorPrograms/MapObjectSystem/Base/MapBase_Object` _array_element_2))
          (`/Game/GameEditor/EditorPrograms/MapObjectSystem/Base/MapBase_Object.UpdateLocation` _asmap_base_object_2))))))

(fn `SetLabelVisible`
  (params (`Show?` :type Boolean)))

(fn `UserConstructionScript`
  (`parent.UserConstructionScript`)
  (bind _returnvalue (`PrimitiveComponent.CreateDynamicMaterialInstance` (`self.DR_X`) 0 "/Game/GameEditor/EditorResources/Materials/Draw/DrawLineMaterial.DrawLineMaterial" "None"))
  (`MaterialInstanceDynamic.SetVectorParameterValue` _returnvalue "Color" (struct :`R` 1.0 :`A` 1.0))
  (bind _returnvalue_2 (`PrimitiveComponent.CreateDynamicMaterialInstance` (`self.DR_Y`) 0 "/Game/GameEditor/EditorResources/Materials/Draw/DrawLineMaterial.DrawLineMaterial" "None"))
  (`MaterialInstanceDynamic.SetVectorParameterValue` _returnvalue_2 "Color" (struct :`G` 1.0 :`A` 1.0))
  (bind _returnvalue_3 (`PrimitiveComponent.CreateDynamicMaterialInstance` (`self.DR_Z`) 0 "/Game/GameEditor/EditorResources/Materials/Draw/DrawLineMaterial.DrawLineMaterial" "None"))
  (`MaterialInstanceDynamic.SetVectorParameterValue` _returnvalue_3 "Color" (struct :`B` 1.0 :`A` 1.0))
  (set `/Game/GameEditor/EditorPrograms/Editor/EditorBaseFunctionController.CurrentTool` 0 (`/Game/GameEditor/EditorPrograms/Editor/MyGameEditorPawn.EditorFunction` (`/Game/GameEditor/EditorPrograms/Editor/FunctionLibrary/GetGamePawn.GetEditorPawn` 0))))