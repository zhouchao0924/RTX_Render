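; Skirting system actor for the map editor's wall system, setting up default skirting and top-skirting line data for rooms.
; BeginPlay starts the model file fetch for the two configured model IDs.
; The callback matches the two response entries by model ID, fills both default line structs and caches model details in the game instance.
; Helpers scan Area actors' adapters for boundaries by room ID or by living/dining room usage name (Chinese strings).
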(event `self.ReceiveBeginPlay`
  (`self.GetSkiringmxFileImplByBlueprint` (`self.SkirtingTemp`)))

(event `self.ReceiveTick`
  (params (DeltaSeconds :type "Float (single-precision)")))

(event `self.GetSkiringmxFileImplByBlueprint`
  (params (InSkirtingNode :type "SkirtingNode Structure (by ref)"))
  (`KismetArrayLibrary.Array_Add` (`self.ModelID`) (`DROperationHouseFunctionLibrary.GetConfigModelIDByType` "EDRSkirtingConfig"))
  (`KismetArrayLibrary.Array_Add` (`self.ModelID`) (`DROperationHouseFunctionLibrary.GetConfigModelIDByType` "EDRTopSkirtingConfig")))

(fn `GetDiningRoomRegion`
  (returns (RoomID :type Integer) (DiningBoundary :type "Array of Vector2D Structure"))
  (locals (TempPs2D :type "Array of Vector2D Structure") (LocalAdapter :type "DRAreaAdapter Object Reference") (LocalPointList :type "Array of Vector Structure"))
  (bind _outactors (`GameplayStatics.GetAllActorsOfClass` "/Game/GameEditor/EditorPrograms/MapWallSystem/Blueprint/Area.Area_C"))
  (if (> (`KismetArrayLibrary.Array_Length` _outactors) 0)
    (for _array_element _outactors
      (bind _returnvalue (`DRProjData.GetAdapter` (`DRProjData.GetProjectDataManager`) (`RoomActor.ObjectID` _array_element)))
      (bind _asdrarea_adapter (cast `DRAreaAdapter` _returnvalue))
      (set `local.LocalAdapter` _asdrarea_adapter)
      (if (`KismetStringLibrary.EqualEqual_StrStr` (`DRAreaAdapter.GetRoomUsageName` (`local.LocalAdapter`)) "餐厅")
        (set `local.LocalPointList` (`/Game/GameEditor/EditorPrograms/MapWallSystem/Blueprint/FunctionLibrary/FunctionLibrary.2DTo3D` (`DRAreaAdapter.GetPointList` (`local.LocalAdapter`))))
        (for _array_element_2 (`local.LocalPointList`)
          (`KismetArrayLibrary.Array_Add` (`local.TempPs2D`) (`KismetMathLibrary.MakeVector2D` (.x _array_element_2) (.y _array_element_2))))
        (return (`DRAreaAdapter.GetRoomID` (`local.LocalAdapter`)) (`local.TempPs2D`))))))

(fn `GetLivingRoomRegion`
  (returns (RoomID :type Integer) (LivingBoundary :type "Array of Vector2D Structure"))
  (locals (TempVec2D :type "Array of Vector2D Structure") (LocalAdapter :type "DRAreaAdapter Object Reference") (LocalPointList :type "Array of Vector Structure"))
  (bind _outactors (`GameplayStatics.GetAllActorsOfClass` "/Game/GameEditor/EditorPrograms/MapWallSystem/Blueprint/Area.Area_C"))
  (if (> (`KismetArrayLibrary.Array_Length` _outactors) 0)
    (for _array_element _outactors
      (bind _returnvalue (`DRProjData.GetAdapter` (`DRProjData.GetProjectDataManager`) (`RoomActor.ObjectID` _array_element)))
      (bind _asdrarea_adapter (cast `DRAreaAdapter` _returnvalue))
      (set `local.LocalAdapter` _asdrarea_adapter)
      (if (`KismetStringLibrary.EqualEqual_StrStr` (`DRAreaAdapter.GetRoomUsageName` (`local.LocalAdapter`)) "客厅")
        (set `local.LocalPointList` (`/Game/GameEditor/EditorPrograms/MapWallSystem/Blueprint/FunctionLibrary/FunctionLibrary.2DTo3D` (`DRAreaAdapter.GetPointList` (`local.LocalAdapter`))))
        (for _array_element_2 (`local.LocalPointList`)
          (`KismetArrayLibrary.Array_Add` (`local.TempVec2D`) (`KismetMathLibrary.MakeVector2D` (.x _array_element_2) (.y _array_element_2))))
        (return (`DRAreaAdapter.GetRoomID` (`local.LocalAdapter`)) (`local.TempVec2D`))))))

(fn `RoomIDMapRegionPs`
  (params (InPutRoomID :type Integer))
  (returns (ReturnValue :type "Array of Vector2D Structure"))
  (locals (LocalAdapter :type "DRAreaAdapter Object Reference"))
  (bind _outactors (`GameplayStatics.GetAllActorsOfClass` "/Game/GameEditor/EditorPrograms/MapWallSystem/Blueprint/Area.Area_C"))
  (if (> (`KismetArrayLibrary.Array_Length` _outactors) 0)
    (for _array_element _outactors
      (bind _returnvalue (`DRProjData.GetAdapter` (`DRProjData.GetProjectDataManager`) (`RoomActor.ObjectID` _array_element)))
      (bind _asdrarea_adapter (cast `DRAreaAdapter` _returnvalue))
      (set `local.LocalAdapter` _asdrarea_adapter)
      (if (== InPutRoomID (`DRAreaAdapter.GetRoomID` (`local.LocalAdapter`)))
        (return (`DRAreaAdapter.GetPointList` (`local.LocalAdapter`)))))))

(fn `SkirtingInfo_Callback`
  (params (NewParam :type "VaRestRequestJSON Object Reference"))
  (locals (IsSkirtingLineModelID :type Integer :default 22506))
  (bind _returnvalue (`VaRestJsonObject.GetObjectArrayField` (`self.data`) "data"))
  (bind _output (`|GetArrayItem` _returnvalue))
  (bind _output_2 (`|GetArrayItem` _returnvalue 1))
  (bind _returnvalue_2 (`VaRestJsonObject.GetStringField` _output_2 "mxFileMD5"))
  (bind _returnvalue_3 (`VaRestJsonObject.GetStringField` _output "mxFileMD5"))
  (bind _returnvalue_4 (`KismetMathLibrary.FTrunc` (`VaRestJsonObject.GetNumberField` _output "skuId")))
  (bind _returnvalue_5 (`KismetMathLibrary.FTrunc` (`VaRestJsonObject.GetNumberField` _output_2 "skuId")))
  (bind _output_3 (`|GetArrayItem` (`VaRestJsonObject.GetObjectArrayField` _output "roomClassList")))
  (bind _output_4 (`|GetArrayItem` (`VaRestJsonObject.GetObjectArrayField` _output_2 "roomClassList")))
  (bind _returnvalue_6 (`KismetMathLibrary.FTrunc` (`VaRestJsonObject.GetNumberField` _output_4 "roomClassId")))
  (bind _returnvalue_7 (`KismetMathLibrary.FTrunc` (`VaRestJsonObject.GetNumberField` _output_3 "roomClassId")))
  (bind _returnvalue_8 (`KismetMathLibrary.FTrunc` (`VaRestJsonObject.GetNumberField` (`|GetArrayItem` (`VaRestJsonObject.GetObjectArrayField` _output_4 "roomCraftList")) "craftId")))
  (bind _returnvalue_9 (`KismetMathLibrary.FTrunc` (`VaRestJsonObject.GetNumberField` (`|GetArrayItem` (`VaRestJsonObject.GetObjectArrayField` _output_3 "roomCraftList")) "craftId")))
  (set `self.data` (`VaRestRequestJSON.GetResponseObject` NewParam))
  (set `local.IsSkirtingLineModelID` (`DROperationHouseFunctionLibrary.GetConfigModelIDByType` "EDRSkirtingConfig"))
  (if (== (`local.IsSkirtingLineModelID`) (`KismetMathLibrary.FTrunc` (`VaRestJsonObject.GetNumberField` _output "modelId")))
    (bind _structout (setmembers `SkirtingLinedefaultNode` :`StructRef` (`self.SkirtingLinedefaultNode`) :`SkirtingMeshModelID` (`DROperationHouseFunctionLibrary.GetConfigModelIDByType` "EDRSkirtingConfig") :`RoomClassID` _returnvalue_7 :`SKUID` _returnvalue_4 :`CraftId` _returnvalue_9 :`SkirtingLineResID` _returnvalue_3))
    (set `self.SkirtingLinedefaultNode` _structout)
    (bind _structout_2 (setmembers `SkirtingLinedefaultNode` :`StructRef` (`self.SkirtingTopLinedefaultNode`) :`SkirtingMeshModelID` (`DROperationHouseFunctionLibrary.GetConfigModelIDByType` "EDRTopSkirtingConfig") :`RoomClassID` _returnvalue_6 :`SKUID` _returnvalue_5 :`CraftId` _returnvalue_8 :`SkirtingLineResID` _returnvalue_2))
    (set `self.SkirtingTopLinedefaultNode` _structout_2)
    (set `self.SkirtingLineResID` (`.SkirtingLineResID` (break `SkirtingLinedefaultNode` (`self.SkirtingLinedefaultNode`))))
    (set `self.SkirtingTopLineResID` (`.SkirtingLineResID` (break `SkirtingLinedefaultNode` (`self.SkirtingTopLinedefaultNode`))))
    (`/Game/GameEditor/EditorPrograms/Editor/EditorGameInstance.AddModelDataToCurrentModelDetailsMap` (`/Game/GameEditor/EditorPrograms/Editor/FunctionLibrary/GetEditorGameInstance.GetEditorGameInstance`) (`DROperationHouseFunctionLibrary.GetConfigModelIDByType` "EDRSkirtingConfig") (`|GetArrayItem` (`VaRestJsonObject.GetObjectArrayField` (`self.data`) "data")))
    (`/Game/GameEditor/EditorPrograms/Editor/EditorGameInstance.AddModelDataToCurrentModelDetailsMap` (`/Game/GameEditor/EditorPrograms/Editor/FunctionLibrary/GetEditorGameInstance.GetEditorGameInstance`) (`DROperationHouseFunctionLibrary.GetConfigModelIDByType` "EDRTopSkirtingConfig") (`|GetArrayItem` (`VaRestJsonObject.GetObjectArrayField` (`self.data`) "data") 1))
    (else
      (bind _structout_3 (setmembers `SkirtingLinedefaultNode` :`StructRef` (`self.SkirtingLinedefaultNode`) :`SkirtingMeshModelID` (`DROperationHouseFunctionLibrary.GetConfigModelIDByType` "EDRSkirtingConfig") :`RoomClassID` _returnvalue_6 :`SKUID` _returnvalue_5 :`CraftId` _returnvalue_8 :`SkirtingLineResID` _returnvalue_2))
      (set `self.SkirtingLinedefaultNode` _structout_3)
      (bind _structout_4 (setmembers `SkirtingLinedefaultNode` :`StructRef` (`self.SkirtingTopLinedefaultNode`) :`SkirtingMeshModelID` (`DROperationHouseFunctionLibrary.GetConfigModelIDByType` "EDRTopSkirtingConfig") :`RoomClassID` _returnvalue_7 :`SKUID` _returnvalue_4 :`CraftId` _returnvalue_9 :`SkirtingLineResID` _returnvalue_3))
      (set `self.SkirtingTopLinedefaultNode` _structout_4)
      (set `self.SkirtingLineResID` (`.SkirtingLineResID` (break `SkirtingLinedefaultNode` (`self.SkirtingLinedefaultNode`))))
      (set `self.SkirtingTopLineResID` (`.SkirtingLineResID` (break `SkirtingLinedefaultNode` (`self.SkirtingTopLinedefaultNode`))))
      (`/Game/GameEditor/EditorPrograms/Editor/EditorGameInstance.AddModelDataToCurrentModelDetailsMap` (`/Game/GameEditor/EditorPrograms/Editor/FunctionLibrary/GetEditorGameInstance.GetEditorGameInstance`) (`DROperationHouseFunctionLibrary.GetConfigModelIDByType` "EDRSkirtingConfig") (`|GetArrayItem` (`VaRestJsonObject.GetObjectArrayField` (`self.data`) "data") 1))
      (`/Game/GameEditor/EditorPrograms/Editor/EditorGameInstance.AddModelDataToCurrentModelDetailsMap` (`/Game/GameEditor/EditorPrograms/Editor/FunctionLibrary/GetEditorGameInstance.GetEditorGameInstance`) (`DROperationHouseFunctionLibrary.GetConfigModelIDByType` "EDRTopSkirtingConfig") (`|GetArrayItem` (`VaRestJsonObject.GetObjectArrayField` (`self.data`) "data"))))))

(fn `UserConstructionScript`)