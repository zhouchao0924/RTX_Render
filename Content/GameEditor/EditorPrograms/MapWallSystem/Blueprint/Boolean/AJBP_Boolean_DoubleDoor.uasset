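; Double-door wall opening for the house editor's map wall system that shows its attribute panel when selected.
; In house-drawing mode the panel goes into the wall main widget; otherwise it goes into the editor pawn's attribute window and is refreshed through Update3DSelect.
; AddUVOffset nudges the selected hole UV from the project data adapter through that panel.
; ShowAttributeIn3D's refresh path casts to the Door panel class, unlike Update3DSelect.
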(event `self.ReceiveBeginPlay`
  (`parent.ReceiveBeginPlay`)
  (add `self.OnSelect` (delegate `OnSelect_Event`)))

(event `OnSelect_Event` :!signature `self.OnSelect`
  (params (isSelect :type Boolean))
  (if (`/Game/GameEditor/EditorPrograms/Editor/EditorGameInstance.IsDrawingHouseMode` (`/Game/GameEditor/EditorPrograms/Editor/FunctionLibrary/GetEditorGameInstance.GetEditorGameInstance`))
    (if isSelect
      (bind _returnvalue (`|CreateWidget` "/Game/GameEditor/EditorPrograms/MapWallSystem/Widget/Boolean/Boolean_Attributes_DoubleDoor.Boolean_Attributes_DoubleDoor_C" null self))
      (`/Game/GameEditor/EditorPrograms/MapWallSystem/Widget/W_WallDrawMainUI.AddAttributes` (`/Game/GameEditor/EditorPrograms/MapWallSystem/Blueprint/FunctionLibrary/FunctionLibrary.GetWallMainWidget`) _returnvalue)
      (else
        (`/Engine/EditorBlueprintResources/StandardMacros.IsValid` _returnvalue
          (:`Is Valid`
            (`Widget.RemoveFromParent` _returnvalue)))))
    (else
      (`self.ShowAttributeIn3D` isSelect))))

(fn `AddUVOffset`
  (params (Delt :type "Float (double-precision)") (UorV :type Boolean))
  (returns (Ret :type Boolean))
  (locals (Local_Delt :type "Float (double-precision)") (Local_UorV :type Boolean) (Local_UV :type "DRUV Structure") (Local_HoleUVs :type "Array of DRUV Structure"))
  (bind _local_delt (`local.Local_Delt`))
  (bind ((`UVOffset` _uvoffset)) (break `DRUV` (`local.Local_UV`)))
  (bind _returnvalue (select `bool` (`local.Local_UorV`) :`false` (+ _uvoffset (`KismetMathLibrary.MakeVector2D` 0.0 _local_delt)) :`true` (+ _uvoffset (`KismetMathLibrary.MakeVector2D` _local_delt))))
  (set `local.Local_Delt` Delt)
  (set `local.Local_UorV` UorV)
  (bind _returnvalue_2 (`DRProjData.GetAdapter` (`DRProjData.GetProjectDataManager`) (`self.ObjectID`)))
  (bind _asdrwindow_hole_adapter (cast `DRWindowHoleAdapter` _returnvalue_2))
  (set `local.Local_HoleUVs` (`DRHoleAdapter.GetHoleUVs` _asdrwindow_hole_adapter))
  (`/Engine/EditorBlueprintResources/StandardMacros.IsValid` (`self.DoorAttributes`)
    (:`Is Valid`
      (bind _asboolean_attributes_double_door (cast `/Game/GameEditor/EditorPrograms/MapWallSystem/Widget/Boolean/Boolean_Attributes_DoubleDoor` (`self.DoorAttributes`))
        (:`then`
          (set `local.Local_UV` (`|GetArrayItem` (`local.Local_HoleUVs`) (`/Game/GameEditor/EditorPrograms/MapWallSystem/Widget/Boolean/Boolean_Attributes_DoubleDoor.SelectIndex` _asboolean_attributes_double_door)))
          (`/Game/GameEditor/EditorPrograms/MapWallSystem/Widget/C_Vector2D.SetValue` (`/Game/GameEditor/EditorPrograms/MapWallSystem/Widget/Boolean/Boolean_Attributes_DoubleDoor.UVOffset` _asboolean_attributes_double_door) _returnvalue)
          (`/Game/UMG/HardBaseAttribute.SetMoveValue` (`/Game/GameEditor/EditorPrograms/MapWallSystem/Widget/Boolean/Boolean_Attributes_DoubleDoor.HardBaseAttribute` _asboolean_attributes_double_door) _returnvalue)
          (return true))
        (:`CastFailed`
          _)))
    (:`Is Not Valid`
      _))
  (return false))

(fn `ShowAttributeIn3D`
  (params (`Select?` :type Boolean))
  (bind _doorattributes (`self.DoorAttributes`))
  (if `Select?`
    (`/Engine/EditorBlueprintResources/StandardMacros.IsValid` (`self.DoorAttributes`)
      (:`Is Valid`
        (bind _asboolean_attributes_door (cast `/Game/GameEditor/EditorPrograms/MapWallSystem/Widget/Boolean/Boolean_Attributes_Door` (`self.DoorAttributes`)))
        (`/Game/GameEditor/EditorPrograms/MapWallSystem/Widget/Boolean/Boolean_Attributes_Door.UpdatebooleanDoorAttribute` _asboolean_attributes_door))
      (:`Is Not Valid`
        (bind _returnvalue (`/Game/GameEditor/EditorPrograms/Widget/C_AttributeWindow.AddAttribute` (`/Game/GameEditor/EditorPrograms/Editor/MyGameEditorPawn.AttributeWindow` (`/Game/GameEditor/EditorPrograms/Editor/FunctionLibrary/GetGamePawn.GetEditorPawn` 0)) "/Game/GameEditor/EditorPrograms/MapWallSystem/Widget/Boolean/Boolean_Attributes_DoubleDoor.Boolean_Attributes_DoubleDoor_C"))
        (bind _output_get (set `self.DoorAttributes` _returnvalue))
        (bind _asboolean_attributes_double_door (cast `/Game/GameEditor/EditorPrograms/MapWallSystem/Widget/Boolean/Boolean_Attributes_DoubleDoor` _output_get))
        (`/Game/GameEditor/EditorPrograms/MapWallSystem/Widget/Boolean/Boolean_Attributes_DoubleDoor.InitBooleanDoubleDoorAttribute` _asboolean_attributes_double_door self)))
    (else
      (`/Engine/EditorBlueprintResources/StandardMacros.IsValid` _doorattributes
        (:`Is Valid`
          (`Widget.RemoveFromParent` _doorattributes)
          (set `self.DoorAttributes` null))))))

(fn `Update3DSelect`
  (returns (Success :type Boolean))
  (if (not (`/Game/GameEditor/EditorPrograms/Editor/EditorGameInstance.IsDrawingHouseMode` (`/Game/GameEditor/EditorPrograms/Editor/FunctionLibrary/GetEditorGameInstance.GetEditorGameInstance`)))
    (`/Engine/EditorBlueprintResources/StandardMacros.IsValid` (`self.DoorAttributes`)
      (:`Is Valid`
        (bind _asboolean_attributes_double_door (cast `/Game/GameEditor/EditorPrograms/MapWallSystem/Widget/Boolean/Boolean_Attributes_DoubleDoor` (`self.DoorAttributes`)))
        (`/Game/GameEditor/EditorPrograms/MapWallSystem/Widget/Boolean/Boolean_Attributes_DoubleDoor.UpDateBooleanDoubleDoorAttribute` _asboolean_attributes_double_door)
        (return true))
      (:`Is Not Valid`
        (bind _returnvalue (`/Game/GameEditor/EditorPrograms/Widget/C_AttributeWindow.AddAttribute` (`/Game/GameEditor/EditorPrograms/Editor/MyGameEditorPawn.AttributeWindow` (`/Game/GameEditor/EditorPrograms/Editor/FunctionLibrary/GetGamePawn.GetEditorPawn` 0)) "/Game/GameEditor/EditorPrograms/MapWallSystem/Widget/Boolean/Boolean_Attributes_DoubleDoor.Boolean_Attributes_DoubleDoor_C"))
        (bind _output_get (set `self.DoorAttributes` _returnvalue))
        (bind _asboolean_attributes_double_door_2 (cast `/Game/GameEditor/EditorPrograms/MapWallSystem/Widget/Boolean/Boolean_Attributes_DoubleDoor` _output_get))
        (`/Game/GameEditor/EditorPrograms/MapWallSystem/Widget/Boolean/Boolean_Attributes_DoubleDoor.InitBooleanDoubleDoorAttribute` _asboolean_attributes_double_door_2 self)
        (return true)))))

(fn `UserConstructionScript`
  (`parent.UserConstructionScript`))