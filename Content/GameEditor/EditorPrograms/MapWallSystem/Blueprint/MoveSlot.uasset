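; MoveSlot is an actor in the editor's map wall system that acts as a slot marker, pairing a Cube with a SlotPoint screen widget.
; The widget is created at BeginPlay unless NObeg is set, recreated on show, and removed on hide or destruction.
; Show and hide events also toggle collision and visibility.
; Tick rescales the flat Cube in proportion to the 2D camera's OrthoWidth, so it tracks zoom.
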(event `隐藏`
  (bind _hud (`self.HUD`))
  (`/Engine/EditorBlueprintResources/StandardMacros.IsValid` _hud
    (:`Is Valid`
      (`Widget.RemoveFromParent` _hud))
    (:`Is Not Valid`
      _))
  (`self.SetActorEnableCollision` false)
  (set `self.Hidden` true))

(event `显示`
  (`self.AddHUD`)
  (`self.SetActorEnableCollision` true)
  (set `self.Hidden` false))

(event `self.ReceiveBeginPlay`
  (if (not (`self.NObeg`))
    (bind _returnvalue (`|CreateWidget` "/Game/GameEditor/EditorPrograms/MapWallSystem/Widget/Draw/SlotPoint.SlotPoint_C" null self :!label _label))
    (set `self.HUD` _returnvalue)
    (`UserWidget.AddToViewport` _returnvalue -10)))

(event `AddHUD`
  (goto _label))

(event `self.ReceiveDestroyed`
  (`/Engine/EditorBlueprintResources/StandardMacros.IsValid` (stale `self.ReceiveBeginPlay` _returnvalue)
    (:`Is Valid`
      (`Widget.RemoveFromParent` (stale `self.ReceiveBeginPlay` _returnvalue))
      (set `self.HUD` null))))

(event `self.ReceiveTick`
  (params (DeltaSeconds :type "Float (single-precision)"))
  (bind _2dcamera (`/Game/GameEditor/EditorPrograms/MapWallSystem/Blueprint/FunctionLibrary/FunctionLibrary.GetPlayer2DCamera` 0))
  (`/Engine/EditorBlueprintResources/StandardMacros.IsValid` _2dcamera
    (:`Is Valid`
      (`SceneComponent.SetWorldScale3D` (`self.Cube`) (`KismetMathLibrary.MakeVector` (.x (`KismetMathLibrary.Conv_DoubleToVector` (/ (/ (`CameraComponent.OrthoWidth` _2dcamera) 1000.0) 15.0))) (.y (`KismetMathLibrary.Conv_DoubleToVector` (/ (/ (`CameraComponent.OrthoWidth` _2dcamera) 1000.0) 15.0))) 0.1)))))

(fn `UserConstructionScript`)