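; Window boolean piece for the map editor's wall system, handling the opening's materials and interior light placement.
; Material functions fill four slots with either a supplied model, room class and crafts, or the wall config defaults on clear.
; InArea probes 15 units to either side, choosing the axis from yaw, and tests the points against Area polygons.
; IRS spawns a horizontal rect light at the matching point, fixed in height and oriented away from the window.
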(event `self.ReceiveBeginPlay`
  (`parent.ReceiveBeginPlay`))

(event `self.ClearMaterial`
  (bind (_roomclass _craft) (`/Game/GameEditor/EditorPrograms/MapWallSystem/Blueprint/FunctionLibrary/FunctionLibrary.GetDefaultRoomClassAndCraft` (`DROperationHouseFunctionLibrary.GetConfigModelIDByType` "EDRWallConfig")))
  (for _index (range 4)
    (`self.SetMaterial` _index null (`DROperationHouseFunctionLibrary.GetConfigModelIDByType` "EDRWallConfig") true null _roomclass (`|MakeArray` _craft))))

(event `self.IRS`
  (bind (_newparam _point) (`self.InArea`))
  (if _newparam
    (`|SpawnActorFromClass` "/Game/HorizontalRectLightActor.HorizontalRectLightActor_C" (`KismetMathLibrary.MakeTransform` (`KismetMathLibrary.MakeVector` (.x _point) (.y _point) 150.0) (`KismetMathLibrary.Conv_VectorToRotator` (`KismetMathLibrary.GetDirectionUnitVector` (`SceneComponent.K2_GetComponentLocation` (`self.B_RootComponent`)) _point))) "Undefined" "OverrideRootScale" null null)))

(fn `InArea`
  (returns (NewParam :type Boolean) (Point :type "Vector Structure"))
  (locals (Local_OnePoint :type "Vector2D Structure"))
  (bind _b_rootcomponent (`self.B_RootComponent`))
  (bind _b_rootcomponent_2 (`self.B_RootComponent`))
  (bind (_x _y) (`KismetMathLibrary.BreakVector2D` (`local.Local_OnePoint`)))
  (bind (_x_2 _y_2) (`KismetMathLibrary.BreakVector2D` (`local.Local_OnePoint`)))
  (bind _returnvalue (`KismetMathLibrary.Abs` (.yaw (`SceneComponent.K2_GetComponentRotation` (`self.B_RootComponent`)))))
  (bind _returnvalue_2 (`KismetMathLibrary.Abs` (.yaw (`SceneComponent.K2_GetComponentRotation` (`self.B_RootComponent`)))))
  (if (or (`KismetMathLibrary.NearlyEqual_FloatFloat` _returnvalue_2 0.0 10.0) (`KismetMathLibrary.NearlyEqual_FloatFloat` _returnvalue_2 180.0 10.0))
    (set `local.Local_OnePoint` (`KismetMathLibrary.MakeVector2D` (.x (+ (`SceneComponent.K2_GetComponentLocation` _b_rootcomponent_2) (0.0 15.0 0.0))) (.y (+ (`SceneComponent.K2_GetComponentLocation` _b_rootcomponent_2) (0.0 15.0 0.0)))))
    (else
      (set `local.Local_OnePoint` (`KismetMathLibrary.MakeVector2D` (.x (+ (`SceneComponent.K2_GetComponentLocation` _b_rootcomponent_2) (15.0 0.0 0.0))) (.y (+ (`SceneComponent.K2_GetComponentLocation` _b_rootcomponent_2) (15.0 0.0 0.0)))))))
  (bind _outactors (`GameplayStatics.GetAllActorsOfClass` "/Game/GameEditor/EditorPrograms/MapWallSystem/Blueprint/Area.Area_C"))
  (for _array_element _outactors
    (bind _returnvalue_3 (`DRProjData.GetAdapter` (`DRProjData.GetProjectDataManager`) (`RoomActor.ObjectID` _array_element)))
    (bind _asdrarea_adapter (cast `DRAreaAdapter` _returnvalue_3))
    (bind _returnvalue_4 (`WallBuildSystem.JudgePointInPolygon` (`/Game/GameEditor/EditorPrograms/MapWallSystem/Blueprint/FunctionLibrary/FunctionLibrary.GetWallSystem` 0) (`/Game/GameEditor/EditorPrograms/MapWallSystem/Blueprint/FunctionLibrary/FunctionLibrary.2DTo3D` (`DRAreaAdapter.GetPointList` _asdrarea_adapter)) (`local.Local_OnePoint`)))
    (if _returnvalue_4
      (return true (`KismetMathLibrary.MakeVector` _x_2 _y_2 (.z (`SceneComponent.K2_GetComponentLocation` (`self.B_RootComponent`)))))))
  (if (or (`KismetMathLibrary.NearlyEqual_FloatFloat` _returnvalue 0.0 10.0) (`KismetMathLibrary.NearlyEqual_FloatFloat` _returnvalue 180.0 10.0))
    (set `local.Local_OnePoint` (`KismetMathLibrary.MakeVector2D` (.x (+ (`SceneComponent.K2_GetComponentLocation` _b_rootcomponent) (0.0 -15.0 0.0))) (.y (+ (`SceneComponent.K2_GetComponentLocation` _b_rootcomponent) (0.0 -15.0 0.0)))))
    (else
      (set `local.Local_OnePoint` (`KismetMathLibrary.MakeVector2D` (.x (+ (`SceneComponent.K2_GetComponentLocation` _b_rootcomponent) (-15.0 0.0 0.0))) (.y (+ (`SceneComponent.K2_GetComponentLocation` _b_rootcomponent) (-15.0 0.0 0.0)))))))
  (bind _outactors_2 (`GameplayStatics.GetAllActorsOfClass` "/Game/GameEditor/EditorPrograms/MapWallSystem/Blueprint/Area.Area_C"))
  (for _array_element_2 _outactors_2
    (bind _returnvalue_5 (`DRProjData.GetAdapter` (`DRProjData.GetProjectDataManager`) (`RoomActor.ObjectID` _array_element_2)))
    (bind _asdrarea_adapter_2 (cast `DRAreaAdapter` _returnvalue_5))
    (bind _returnvalue_6 (`WallBuildSystem.JudgePointInPolygon` (`/Game/GameEditor/EditorPrograms/MapWallSystem/Blueprint/FunctionLibrary/FunctionLibrary.GetWallSystem` 0) (`/Game/GameEditor/EditorPrograms/MapWallSystem/Blueprint/FunctionLibrary/FunctionLibrary.2DTo3D` (`DRAreaAdapter.GetPointList` _asdrarea_adapter_2)) (`local.Local_OnePoint`)))
    (if _returnvalue_6
      (return true (`KismetMathLibrary.MakeVector` _x _y (.z (`SceneComponent.K2_GetComponentLocation` (`self.B_RootComponent`))))))))

(fn `Set WindowBooleanMaterialDependsArea`
  (params (ModelId :type Integer) (Crafts :type "Array of Integer") (RoomClassID :type Integer))
  (locals (`Local Model Id` :type Integer) (`Local Crafts` :type "Array of Integer") (`Local RoomClassID` :type Integer))
  (set `local.Local Model Id` ModelId)
  (set `local.Local Crafts` Crafts)
  (set `local.Local RoomClassID` RoomClassID)
  (for _index (range 4)
    (`self.SetMaterial` _index null (`local.Local Model Id`) true null (`local.Local RoomClassID`) (`local.Local Crafts`))))

(fn `UserConstructionScript`
  (`parent.UserConstructionScript`))