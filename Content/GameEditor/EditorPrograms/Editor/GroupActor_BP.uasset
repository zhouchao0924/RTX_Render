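; GroupActor_BP is an editor actor that groups placed map objects so they can be attached, copied or released together.
; Membership lives as model tags in GroupInfo, which Init matches against level actors to rebuild GroupActors and parent back-references.
; Add accepts nested groups, Polymerization attaches members recursively, and removing the last object destroys the group.
; Copy re-creates models through project data adapters into a newly spawned, re-tagged group.
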(fn `AddActorToGroup`
  (params (Target :type "Actor Object Reference"))
  (returns (ReturnValue :type Boolean))
  (locals (LocalTargetActor :type "Actor Object Reference") (LocalCurrentMapBase_Object :type "/Game/GameEditor/EditorPrograms/MapObjectSystem/Base/MapBase_Object Object Reference") (LocalCurrentGroupActor :type "GroupActorBase Object Reference") (LocalCurrentTag :type String) (LocalCurrentChildTags :type "Array of String") (Local_ModelAdapter :type "DRModelInstanceAdapter Object Reference"))
  (set `local.LocalTargetActor` Target)
  (`/Engine/EditorBlueprintResources/StandardMacros.IsValid` (`local.LocalTargetActor`)
    (:`Is Valid`
      (if (`KismetArrayLibrary.Array_Contains` (`self.GroupActors`) (`local.LocalTargetActor`))
        (return true)
        (else
          (bind _asmap_base_object (cast `/Game/GameEditor/EditorPrograms/MapObjectSystem/Base/MapBase_Object` (`local.LocalTargetActor`))
            (:`then`
              (set `local.LocalCurrentMapBase_Object` _asmap_base_object)
              (`KismetArrayLibrary.Array_Add` (`/Game/GameEditor/EditorPrograms/MapObjectSystem/Base/MapBase_Object.GroupParentReference` (`local.LocalCurrentMapBase_Object`)) self)
              (bind _returnvalue (`DRProjData.GetAdapter` (`DRProjData.GetProjectDataManager`) (`FurnitureModelActor.ObjectId` (`local.LocalCurrentMapBase_Object`))))
              (bind _asdrmodel_instance_adapter (cast `DRModelInstanceAdapter` _returnvalue))
              (set `local.Local_ModelAdapter` _asdrmodel_instance_adapter)
              (set `local.LocalCurrentTag` (`DRModelInstanceAdapter.GetModelTag` (`local.Local_ModelAdapter`))))
            (:`CastFailed`
              (bind _asgroup_actor_base (cast `GroupActorBase` (`local.LocalTargetActor`))
                (:`then`
                  (set `local.LocalCurrentGroupActor` _asgroup_actor_base)
                  (`KismetArrayLibrary.Array_Add` (`GroupActorBase.GroupParentReference` (`local.LocalCurrentGroupActor`)) self)
                  (set `local.LocalCurrentTag` (`.GroupSelfTag` (break `GroupActorInfo` (`GroupActorBase.GroupInfo` (`local.LocalCurrentGroupActor`))))))
                (:`CastFailed`
                  (return false)))))
          (set `local.LocalCurrentChildTags` (`.GroupChildTag` (break `GroupActorInfo` (`self.GroupInfo`))))
          (`KismetArrayLibrary.Array_Add` (`local.LocalCurrentChildTags`) (`local.LocalCurrentTag`))
          (setmembers `GroupActorInfo` :`StructRef` (`self.GroupInfo`) :`GroupChildTag` (`local.LocalCurrentChildTags`))
          (`KismetArrayLibrary.Array_Add` (`self.GroupActors`) (`local.LocalTargetActor`))
          (return true))))
    (:`Is Not Valid`
      (return false))))

(fn `CheckGroupIsCollection`
  (locals (Local_Model :type "/Game/GameEditor/EditorPrograms/MapObjectSystem/Base/MapBase_Object Object Reference") (Local_CheckIsCollectionJson :type "VaRestJsonObject Object Reference")))

(fn `CheckGroupIsCollection_CallBack`
  (params (Request :type "VaRestRequestJSON Object Reference"))
  (locals (LocalRequestJson :type "VaRestJsonObject Object Reference") (Local_CollectionId :type String))
  (bind _returnvalue (`VaRestJsonObject.GetStringField` (`local.LocalRequestJson`) "data"))
  (set `local.LocalRequestJson` (`VaRestRequestJSON.GetResponseObject` Request))
  (if (`VaRestJsonObject.GetBoolField` (`local.LocalRequestJson`) "success")
    (set `local.Local_CollectionId` _returnvalue)
    (if (`KismetStringLibrary.NotEqual_StrStr` _returnvalue)
      (set `self.CollectionId` (`local.Local_CollectionId`))
      (else
        (set `self.CollectionId` "")))))

(fn `Clean`
  (returns (ReturnValue :type Boolean))
  (locals (LocalCurrentActor :type "Actor Object Reference") (LocalCurrentModel :type "/Game/GameEditor/EditorPrograms/MapObjectSystem/Base/MapBase_Object Object Reference") (LocalGroupActors :type "Array of Actor Object Reference"))
  (set `local.LocalGroupActors` (`self.GroupActors`))
  (for _array_element (`local.LocalGroupActors`)
    (set `local.LocalCurrentActor` _array_element)
    (`/Engine/EditorBlueprintResources/StandardMacros.IsValid` (`local.LocalCurrentActor`)
      (:`Is Valid`
        (bind _asmap_base_object (cast `/Game/GameEditor/EditorPrograms/MapObjectSystem/Base/MapBase_Object` (`local.LocalCurrentActor`)))
        (set `local.LocalCurrentModel` _asmap_base_object)
        (`self.RemoveActorFromGroup` (`local.LocalCurrentModel`)))))
  (`KismetArrayLibrary.Array_Clear` (`self.GroupActors`))
  (`self.K2_DestroyActor`)
  (return true))

(fn `Copy`
  (returns (ReturnValue :type "Array of Actor Object Reference"))
  (locals (LocalCurrentModel :type "/Game/GameEditor/EditorPrograms/MapObjectSystem/Base/MapBase_Object Object Reference") (LocalSpawnedActor :type "/Game/GameEditor/EditorPrograms/MapObjectSystem/Base/MapBase_Object Object Reference") (LocalNewId :type Integer :default 0) (LocalSpawnedList :type "Array of Actor Object Reference") (LocalSpawnedGroup :type "/Game/GameEditor/EditorPrograms/Editor/GroupActor_BP Object Reference") (LocalSpawnedTagList :type "Array of String") (LocalNewTag :type String) (Local_ModelAdapter :type "DRModelInstanceAdapter Object Reference") (Local_UV :type "DRUV Structure") (Local_ObjId :type Integer :default 0) (Local_AllObjId :type "Array of Integer"))
  (bind (_seconds _partialseconds) (`GameplayStatics.GetAccurateRealTime`))
  (bind (_seconds_2 _partialseconds_2) (`GameplayStatics.GetAccurateRealTime`))
  (bind (_outnormalmodeldata _returnvalue) (`DROperationBuildingFunctionLibrary.ConvertModelAdapterToNormalModel` (`FurnitureModelActor.ObjectId` (`local.LocalCurrentModel`))))
  (bind (_value _returnvalue_2) (`BlueprintMapLibrary.Map_Find` (`DRProjData.NormalModelMap` (`DRProjData.GetProjectDataManager`)) (`local.Local_ObjId`)))
  (for _array_element (`self.GroupActors`)
    (bind _asmap_base_object (cast `/Game/GameEditor/EditorPrograms/MapObjectSystem/Base/MapBase_Object` _array_element))
    (set `local.LocalCurrentModel` _asmap_base_object)
    (if _returnvalue
      (bind _structout (setmembers `DNormalModel` :`StructRef` _outnormalmodeldata :`ModelTag` ""))
      (bind _returnvalue_3 (`DROperationBuildingFunctionLibrary.AddNewModel` _structout))
      (set `local.Local_ObjId` _returnvalue_3)
      (`KismetArrayLibrary.Array_Add` (`local.Local_AllObjId`) (`local.Local_ObjId`))))
  (bind _returnvalue_4 (`|SpawnActorFromClass` "GroupActor_BP_C" (`self.GetTransform`) "Undefined" "OverrideRootScale" null (`self.GroupInfo`) null))
  (set `local.LocalSpawnedGroup` _returnvalue_4)
  (bind _returnvalue_5 (`CEditorGameInstance.GetBuildingSystemInstance` (`/Game/GameEditor/EditorPrograms/Editor/FunctionLibrary/GetEditorGameInstance.GetEditorGameInstance`)))
  (`BuildingSystem.ForceUpdateSuit` _returnvalue_5)
  (for _array_element_2 (`local.Local_AllObjId`)
    (set `local.Local_ObjId` _array_element_2)
    (if _returnvalue_2
      (bind _asmap_base_object_2 (cast `/Game/GameEditor/EditorPrograms/MapObjectSystem/Base/MapBase_Object` _value))
      (set `local.LocalSpawnedActor` _asmap_base_object_2)
      (bind _returnvalue_6 (`DRProjData.GetAdapter` (`DRProjData.GetProjectDataManager`) (`local.Local_ObjId`)))
      (bind _asdrmodel_instance_adapter (cast `DRModelInstanceAdapter` _returnvalue_6))
      (set `local.Local_ModelAdapter` _asdrmodel_instance_adapter)
      (set `local.LocalNewTag` (`DRModelInstanceAdapter.GetModelTag` (`local.Local_ModelAdapter`)))
      (if (`LuoLuoBlueprintFunctionLibrary.IsEmpty` (`local.LocalNewTag`))
        (set `local.LocalNewTag` (`KismetStringLibrary.Concat_StrStr` (`KismetSystemLibrary.GetObjectName` (`local.LocalSpawnedActor`)) "_" (`KismetStringLibrary.Conv_DoubleToString` (+ (`KismetMathLibrary.Conv_IntToDouble` _seconds_2) _partialseconds_2))))
        (`DRModelInstanceAdapter.SetModelTag` (`local.Local_ModelAdapter`) (`local.LocalNewTag`)))
      (`KismetArrayLibrary.Array_Add` (`local.LocalSpawnedTagList`) (`local.LocalNewTag`))
      (`KismetArrayLibrary.Array_Add` (`local.LocalSpawnedList`) (`local.LocalSpawnedActor`))))
  (setmembers `GroupActorInfo` :`StructRef` (`GroupActorBase.GroupInfo` (`local.LocalSpawnedGroup`)) :`GroupSelfTag` (`KismetStringLibrary.Concat_StrStr` (`KismetSystemLibrary.GetObjectName` (`local.LocalSpawnedGroup`)) "_" (`KismetStringLibrary.Conv_DoubleToString` (+ (`KismetMathLibrary.Conv_IntToDouble` _seconds) _partialseconds))) :`GroupChildTag` (`local.LocalSpawnedTagList`))
  (set `GroupActorBase.GroupActors` (`local.LocalSpawnedList`) (`local.LocalSpawnedGroup`))
  (return (`local.LocalSpawnedList`)))

(fn `GetGroupModelIdList`
  (returns (ModelIdList :type "Array of Float (double-precision)"))
  (locals (Local_ModelAdapter :type "DRModelInstanceAdapter Object Reference") (Local_Model :type "/Game/GameEditor/EditorPrograms/MapObjectSystem/Base/MapBase_Object Object Reference") (Local_ModelIdList :type "Array of Float (double-precision)"))
  (for _array_element (`.GroupChildTag` (break `GroupActorInfo` (`self.GroupInfo`)))
    (bind _outactors (`GameplayStatics.GetAllActorsWithTag` (`KismetStringLibrary.Conv_StringToName` _array_element)))
    (bind _asmap_base_object (cast `/Game/GameEditor/EditorPrograms/MapObjectSystem/Base/MapBase_Object` (`|GetArrayItem` _outactors)))
    (set `local.Local_Model` _asmap_base_object)
    (bind _returnvalue (`DRProjData.GetAdapter` (`DRProjData.GetProjectDataManager`) (`FurnitureModelActor.ObjectId` (`local.Local_Model`))))
    (bind _asdrmodel_instance_adapter (cast `DRModelInstanceAdapter` _returnvalue))
    (set `local.Local_ModelAdapter` _asdrmodel_instance_adapter)
    (`KismetArrayLibrary.Array_Add` (`local.Local_ModelIdList`) (`KismetMathLibrary.Conv_IntToDouble` (`DRModelInstanceAdapter.GetModelID` (`local.Local_ModelAdapter`)))))
  (return (`local.Local_ModelIdList`)))

(fn `Init`
  (returns (ReturnValue :type Boolean))
  (locals (LocalInitActorList :type "Array of Actor Object Reference") (LocalCurrentMapBase_Object :type "/Game/GameEditor/EditorPrograms/MapObjectSystem/Base/MapBase_Object Object Reference") (LocalSuccess :type Boolean :default true) (LocalCurrentTag :type String) (LocalCurrentGroupActor :type "GroupActorBase Object Reference") (LocalCurrentActor :type "Actor Object Reference") (LocalCustomCurtain :type "/Game/GameEditor/EditorPrograms/MapObjectSystem/S_CustomModel/MapBase_CustomCurtain Object Reference") (Local_ModelAdapter :type "DRModelInstanceAdapter Object Reference"))
  (bind _outactors (`GameplayStatics.GetAllActorsOfClass` "/Script/Engine.Actor"))
  (set `local.LocalInitActorList` _outactors)
  (for _array_element (`local.LocalInitActorList`)
    (set `local.LocalCurrentActor` _array_element)
    (if (!= (`local.LocalCurrentActor`) self)
      (cast `/Game/GameEditor/EditorPrograms/MapObjectSystem/S_Light/MapBase_LightModel` (`local.LocalCurrentActor`)
        (:`CastFailed`
          (cast `/Game/GameEditor/EditorPrograms/MapObjectSystem/S_Model/MapBase_InstallModel` (`local.LocalCurrentActor`)
            (:`CastFailed`
              (bind _asmap_base_object (cast `/Game/GameEditor/EditorPrograms/MapObjectSystem/Base/MapBase_Object` (`local.LocalCurrentActor`)))
              (set `local.LocalCurrentMapBase_Object` _asmap_base_object)
              (if (not (`/Game/GameEditor/EditorPrograms/MapObjectSystem/Base/MapBase_Object.IsDoorAndWindow` (`local.LocalCurrentMapBase_Object`)))
                (bind _asmap_base_custom_curtain (cast `/Game/GameEditor/EditorPrograms/MapObjectSystem/S_CustomModel/MapBase_CustomCurtain` (`local.LocalCurrentMapBase_Object`))
                  (:`then`
                    (set `local.LocalCustomCurtain` _asmap_base_custom_curtain)
                    (set `local.LocalCurrentTag` (`.ModelTag` (break `CustomCurtainSaved` (`/Game/GameEditor/EditorPrograms/MapObjectSystem/S_CustomModel/MapBase_CustomCurtain.CustomCurtainInfo` (`local.LocalCustomCurtain`))))))
                  (:`CastFailed`
                    (bind _returnvalue (`DRProjData.GetAdapter` (`DRProjData.GetProjectDataManager`) (`FurnitureModelActor.ObjectId` (`local.LocalCurrentMapBase_Object`))))
                    (bind _asdrmodel_instance_adapter (cast `DRModelInstanceAdapter` _returnvalue))
                    (set `local.Local_ModelAdapter` _asdrmodel_instance_adapter)
                    (set `local.LocalCurrentTag` (`DRModelInstanceAdapter.GetModelTag` (`local.Local_ModelAdapter`)))))
                (if (`KismetArrayLibrary.Array_Contains` (`.GroupChildTag` (break `GroupActorInfo` (`self.GroupInfo`))) (`local.LocalCurrentTag`))
                  (`KismetArrayLibrary.Array_Add` (`/Game/GameEditor/EditorPrograms/MapObjectSystem/Base/MapBase_Object.GroupParentReference` (`local.LocalCurrentMapBase_Object`)) self)
                  (`KismetArrayLibrary.Array_Add` (`self.GroupActors`) (`local.LocalCurrentMapBase_Object`))
                  (else
                    (set `local.LocalSuccess` false))))))))))
  (`self.CheckGroupIsCollection`)
  (return (`local.LocalSuccess`)))

(fn `Polymerization`
  (returns (ReturnValue :type Boolean))
  (locals (LocalGroupActor :type "Actor Object Reference"))
  (for _array_element (`self.GroupActors`)
    (set `local.LocalGroupActor` _array_element)
    (bind _asgroup_actor_base (cast `GroupActorBase` (`local.LocalGroupActor`))
      (:`then`
        (`self.Polymerization` _asgroup_actor_base))
      (:`CastFailed`
        (bind _as3dgame_mode (cast `/Game/GameEditor/EditorPrograms/Editor/3DGameMode` (`GameplayStatics.GetGameMode`))
          (:`then`
            (`KismetArrayLibrary.Array_AddUnique` (`/Game/GameEditor/EditorPrograms/Editor/3DGameMode.SelectedGroupActors` _as3dgame_mode) (`local.LocalGroupActor`)))
          (:`CastFailed`
            _))))
    (`self.K2_AttachToActor` (`local.LocalGroupActor`) self "None" "KeepWorld" "KeepWorld" "KeepWorld" true)
    (`/Game/GameEditor/EditorPrograms/Editor/FunctionLibrary/SetActorRender.SetActorRender` (`local.LocalGroupActor`) true))
  (return true))

(fn `RemoveActorFromGroup`
  (params (Target :type "Actor Object Reference"))
  (returns (ReturnValue :type Boolean))
  (locals (LocalRemoveActor :type "Actor Object Reference") (LocalRemoveMapBase_Object :type "/Game/GameEditor/EditorPrograms/MapObjectSystem/Base/MapBase_Object Object Reference") (LocalChildTags :type "Array of String") (Local_ModelAdapter :type "DRModelInstanceAdapter Object Reference"))
  (set `local.LocalRemoveActor` Target)
  (`KismetArrayLibrary.Array_RemoveItem` (`self.GroupActors`) (`local.LocalRemoveActor`))
  (bind _asmap_base_object (cast `/Game/GameEditor/EditorPrograms/MapObjectSystem/Base/MapBase_Object` (`local.LocalRemoveActor`))
    (:`then`
      (set `local.LocalRemoveMapBase_Object` _asmap_base_object)
      (`KismetArrayLibrary.Array_RemoveItem` (`/Game/GameEditor/EditorPrograms/MapObjectSystem/Base/MapBase_Object.GroupParentReference` (`local.LocalRemoveMapBase_Object`)) self)
      (set `local.LocalChildTags` (`.GroupChildTag` (break `GroupActorInfo` (`self.GroupInfo`))))
      (bind _returnvalue (`DRProjData.GetAdapter` (`DRProjData.GetProjectDataManager`) (`FurnitureModelActor.ObjectId` (`local.LocalRemoveMapBase_Object`))))
      (bind _asdrmodel_instance_adapter (cast `DRModelInstanceAdapter` _returnvalue))
      (set `local.Local_ModelAdapter` _asdrmodel_instance_adapter)
      (`KismetArrayLibrary.Array_RemoveItem` (`local.LocalChildTags`) (`DRModelInstanceAdapter.GetModelTag` (`local.Local_ModelAdapter`)))
      (setmembers `GroupActorInfo` :`StructRef` (`self.GroupInfo`) :`GroupChildTag` (`local.LocalChildTags`))
      (bind _asgroup_actor_bp (cast `/Game/GameEditor/EditorPrograms/Editor/GroupActor_BP` (`self.GetParentActor` (`local.LocalRemoveActor`)))
        (:`then`
          (`self.K2_DetachFromActor` _asgroup_actor_bp "KeepWorld" "KeepWorld" "KeepWorld"))
        (:`CastFailed`
          _))
      (if (not (`KismetArrayLibrary.Array_IsValidIndex` (`self.GroupActors`)))
        (`self.K2_DestroyActor`))
      (return true))
    (:`CastFailed`
      (return false))))

(fn `RemoveAttribute`)

(fn `Select`
  (params (bFromUI :type Boolean))
  (returns (ReturnValue :type Boolean))
  (locals (LocalSelectFromUI :type Boolean :default false)))

(fn `SetGroupActorPosition`
  (returns (ReturnValue :type Boolean))
  (locals (Local_TempActorList :type "Array of Vector Structure") (Local_NewPos :type "Vector Structure" :default (0.0 0.0 0.0)))
  (for _array_element (`self.GroupActors`)
    (`KismetArrayLibrary.Array_Add` (`local.Local_TempActorList`) (`self.K2_GetActorLocation` _array_element))
    (`self.K2_DetachFromActor` _array_element "KeepWorld" "KeepWorld" "KeepWorld")))

(fn `UserConstructionScript`)