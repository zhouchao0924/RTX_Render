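; AreaPlane is a map wall system actor in the game editor that builds procedural floor and roof surfaces for an area from a shared vertex list.
; On BeginPlay it creates the ground mesh, then rewrites vertex Z around Height to create two roof layers, only the upper receiving normals.
; All three meshes share one area material.
; A normal-scaling helper and a resource-based material lookup exist but are unused.
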(event `self.ReceiveBeginPlay`
  (bind _verlist (`self.VerList`))
  (bind _verlist_2 (`self.VerList`))
  (bind _verlist_3 (`self.VerList`))
  (bind _triangles (`self.Triangles`))
  (bind _uvo (`self.UVO`))
  (`ProceduralMeshComponent.CreateMeshSection_LinearColor` :`self` (`self.Pround`) :`Vertices` _verlist :`Triangles` _triangles :`UV0` _uvo)
  (for (_array_element _array_index) _verlist_2
    (`KismetArrayLibrary.Array_Set` _verlist_2 _array_index (`KismetMathLibrary.MakeVector` (.x _array_element) (.y _array_element) (- (`self.Height`) 10.0))))
  (`ProceduralMeshComponent.CreateMeshSection_LinearColor` :`self` (`self.Roof`) :`Vertices` _verlist :`Triangles` _triangles :`UV0` _uvo)
  (for (_array_element_2 _array_index_2) _verlist_3
    (`KismetArrayLibrary.Array_Set` _verlist_3 _array_index_2 (`KismetMathLibrary.MakeVector` (.x _array_element_2) (.y _array_element_2) (+ (`self.Height`) 0.1))))
  (`ProceduralMeshComponent.CreateMeshSection_LinearColor` :`self` (`self.Roof2`) :`Vertices` (`self.VerList`) :`Triangles` (`self.Triangles`) :`Normals` (`self.Normals`) :`UV0` (`self.UVO`))
  (`PrimitiveComponent.SetMaterial` (`self.Roof`) 0 "/Game/GameEditor/EditorPrograms/MapWallSystem/Material/AreaPlaneMaterial.AreaPlaneMaterial")
  (`PrimitiveComponent.SetMaterial` (`self.Roof2`) 0 "/Game/GameEditor/EditorPrograms/MapWallSystem/Material/AreaPlaneMaterial.AreaPlaneMaterial")
  (`PrimitiveComponent.SetMaterial` (`self.Pround`) 0 "/Game/GameEditor/EditorPrograms/MapWallSystem/Material/AreaPlaneMaterial.AreaPlaneMaterial"))

(fn `NormalReverse`
  (params (VectorNormal :type "Array of Vector Structure") (Normalvector :type "Vector Structure"))
  (returns (Out :type "Array of Vector Structure"))
  (bind _vnormals (`self.VNormals`))
  (for _array_element VectorNormal
    (`KismetArrayLibrary.Array_Add` _vnormals (* _array_element Normalvector)))
  (return _vnormals))

(fn `UserConstructionScript`)