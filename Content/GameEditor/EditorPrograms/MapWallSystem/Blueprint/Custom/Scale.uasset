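; Map editor actor in the wall system for interactively scaling and rotating a plane with the mouse.
; F detaches pivot and plane: point A follows the cursor until click, point B until release, storing their baseline distance.
; After reattaching, Tick keeps B on the cursor, scaling pivot X/Y by current-to-baseline distance, with debug drawing.
; A MoveSlot handle spawned on BeginPlay steers actor yaw, snapping near right angles.
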(event `SetScale`
  (bind _worldlocation (`PlayerController.DeprojectMousePositionToWorld` (`GameplayStatics.GetPlayerController` 0)))
  (bind _returnvalue (`PlayerController.IsInputKeyDown` (`GameplayStatics.GetPlayerController` 0) "LeftMouseButton"))
  (bind _returnvalue_2 (- (`SceneComponent.K2_GetComponentLocation` (`self.Scene`)) (`SceneComponent.K2_GetComponentLocation` (`self.S`))))
  (set `self.StartSetScale` true)
  (`SceneComponent.K2_DetachFromComponent` (`self.Plane`) "KeepWorld" "KeepWorld" "KeepWorld" true)
  (`SceneComponent.K2_DetachFromComponent` (`self.Scene`) "KeepWorld" "KeepWorld" "KeepWorld" true)
  (if _returnvalue :!label _label
    (if _returnvalue :!label _label_2
      (`SceneComponent.K2_SetWorldLocation` (`self.S`) _worldlocation false false)
      (`KismetSystemLibrary.Delay` 0.0)
      (goto _label_2)
      (else
        (set `self.offset` _returnvalue_2)
        (set `self.o` (`KismetMathLibrary.VSize` _returnvalue_2))
        (`SceneComponent.K2_AttachToComponent` (`self.Scene`) (`self.K2_GetRootComponent`) "None" "KeepWorld" "KeepWorld" "KeepWorld" true)
        (`SceneComponent.K2_AttachToComponent` (`self.Plane`) (`self.Scene`) "None" "KeepWorld" "KeepWorld" "KeepWorld" true)
        (set `self.StartSetScale` false)
        (set `self.StartTick` true)))
    (else
      (`SceneComponent.K2_SetWorldLocation` (`self.Scene`) _worldlocation false false)
      (if (`self.StartSetScale`)
        (`KismetSystemLibrary.Delay` 0.0)
        (goto _label)))))

(event `Key|F`
  (params (Key :type "Key Structure" :default "AnyKey"))
  (:`Pressed`
    (`self.SetScale`)))

(event `self.ReceiveBeginPlay`
  (`self.Select` true))

(event `Select`
  (params (IsSelect :type Boolean))
  (if IsSelect
    (bind _returnvalue (`PeExtendedToolKitBPLibrary.SpawnActor` "/Game/GameEditor/EditorPrograms/MapWallSystem/Blueprint/MoveSlot.MoveSlot_C" (`SceneComponent.K2_GetComponentLocation` (`self.RotaSlot`)) (struct)))
    (set `self.RotationSlot` _returnvalue)))

(event `self.ReceiveTick`
  (params (DeltaSeconds :type "Float (single-precision)"))
  (bind _returnvalue (`SceneComponent.K2_GetComponentLocation` (`self.Scene`)))
  (bind _returnvalue_2 (/ (`self.o`) 100.0))
  (bind _returnvalue_3 (`SceneComponent.K2_GetComponentLocation` (`self.S`)))
  (bind _yaw (.yaw (`KismetMathLibrary.Conv_VectorToRotator` (- (`self.K2_GetActorLocation` (`self.RotationSlot`)) (`self.K2_GetActorLocation`)))))
  (bind _returnvalue_4 (+ (/ (- (`KismetMathLibrary.VSize` (/ (- (`SceneComponent.K2_GetComponentLocation` (`self.S`)) (`SceneComponent.K2_GetComponentLocation` (`self.Scene`))) 100.0)) _returnvalue_2) _returnvalue_2) 1.0))
  (bind _returnvalue_5 (`KismetMathLibrary.MakeVector` _returnvalue_4 _returnvalue_4 1.0))
  (`|ExecutionSequence`
    (:`then_0`
      (`KismetSystemLibrary.DrawDebugString` _returnvalue "缩放点A" null (struct :`G` 0.08642 :`B` 1.0 :`A` 1.0))
      (`KismetSystemLibrary.DrawDebugString` _returnvalue_3 "缩放点B" null (struct :`R` 1.0 :`G` 0.027614 :`A` 1.0))
      (`KismetSystemLibrary.DrawDebugLine` _returnvalue _returnvalue_3 (struct :`R` 0.889569 :`B` 1.0 :`A` 1.0)))
    (:`then_1`
      (`/Engine/EditorBlueprintResources/StandardMacros.IsValid` (`self.RotationSlot`)
        (:`Is Valid`
          (`self.K2_SetActorRotation` (`KismetMathLibrary.MakeRotator` 0.0 0.0 (select `bool` (`KismetMathLibrary.NearlyEqual_FloatFloat` _yaw -90.0 10.0) :`false` (select `bool` (`KismetMathLibrary.NearlyEqual_FloatFloat` _yaw 180.0 10.0) :`false` (select `bool` (`KismetMathLibrary.NearlyEqual_FloatFloat` _yaw 90.0 10.0) :`false` (select `bool` (`KismetMathLibrary.NearlyEqual_FloatFloat` _yaw 0.0 10.0) :`false` _yaw) :`true` 90.0) :`true` 180.0) :`true` -90.0))))))
    (:`then_2`
      (if (`self.StartTick`)
        (`SceneComponent.SetRelativeScale3D` (`self.Scene`) _returnvalue_5)
        (`PeExtendedToolKitBPLibrary.PrintOut` (`KismetStringLibrary.Conv_VectorToString` _returnvalue_5))
        (`SceneComponent.K2_SetWorldLocation` (`self.S`) (`PlayerController.DeprojectMousePositionToWorld` (`GameplayStatics.GetPlayerController` 0)) false false)))))

(fn `UserConstructionScript`)