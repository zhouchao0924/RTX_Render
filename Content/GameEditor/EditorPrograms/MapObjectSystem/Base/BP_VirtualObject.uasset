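; BP_VirtualObject is a map editor placeholder that shows a model in a virtual material until its spawn actor overlaps it.
; It loads the model by MD5 resource ID, caches original materials and binds overlap events.
; Overlap hides the spawn actor, shows editor tips and restores original materials.
; The editor pawn's overlap list keeps the latest placeholder highlighted, reverting to the previous on exit or unhiding the actor when none remain.
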(event `self.ReceiveBeginPlay`
  ;[1 1 1] start
  (`self.Init`))

(event `UpdateModel`
  (params (Resource :type "Resource Object Reference"))
  (bind _modelfile (`self.ModelFile`))
  ;[1 1 1] UpdateModel,OverlapEvent
  (bind _asmodel_file (cast `ModelFile` Resource))
  (`Resource.ForceLoad` _asmodel_file)
  (add `ModelFileComponent.UpdateModelDone` _modelfile (delegate `UpdateModelDone`))
  (`ModelFileComponent.UpdateModel` _modelfile _asmodel_file))

(event `UpdateModelDone`
  ;[1 1 1] UpdateModel,OverlapEvent
  (bind _returnvalue (`ModelFileComponent.GetPart` (`self.ModelFile`) 0))
  (`/Engine/EditorBlueprintResources/StandardMacros.IsValid` _returnvalue
    (:`Is Valid`
      (set `self.OriginalMaterials` (`MeshComponent.GetMaterials` _returnvalue))
      (`self.SetVirtualMaterial`)
      (`PrimitiveComponent.SetCollisionProfileName` _returnvalue "OverlapAll")
      (add `PrimitiveComponent.OnComponentBeginOverlap` _returnvalue (delegate `BeginOverlap`))
      (add `PrimitiveComponent.OnComponentEndOverlap` _returnvalue (delegate `EndOverlap`)))))

(event `EndOverlap`
  (params (OverlappedComponent :type "PrimitiveComponent Object Reference") (OtherActor :type "Actor Object Reference") (OtherComp :type "PrimitiveComponent Object Reference") (OtherBodyIndex :type Integer))
  ;[1 1 1] UpdateModel,OverlapEvent
  (if (`/Game/GameEditor/EditorPrograms/MapWallSystem/Blueprint/FunctionLibrary/FunctionLibrary.==` OtherActor (`self.SpawnActor`))
    (`/Game/GameEditor/EditorPrograms/Editor/MyGameEditorPawn.CreateVirtualTips` (`/Game/GameEditor/EditorPrograms/Editor/FunctionLibrary/GetGamePawn.GetEditorPawn` 0) false)
    (`self.ManageOverlapedList` false OtherActor)
    (`self.SetVirtualMaterial`)))

(event `BeginOverlap`
  (params (OverlappedComponent :type "PrimitiveComponent Object Reference") (OtherActor :type "Actor Object Reference") (OtherComp :type "PrimitiveComponent Object Reference") (OtherBodyIndex :type Integer) (bFromSweep :type Boolean) (SweepResult :type "HitResult Structure (by ref)"))
  ;[1 1 1] UpdateModel,OverlapEvent
  (if (`/Game/GameEditor/EditorPrograms/MapWallSystem/Blueprint/FunctionLibrary/FunctionLibrary.==` OtherActor (`self.SpawnActor`))
    (`self.BeginOverLapEvent` OtherActor)))

(fn `BeginOverLapEvent`
  (params (Actor :type "Actor Object Reference"))
  (bind _asmap_base_object (cast `/Game/GameEditor/EditorPrograms/MapObjectSystem/Base/MapBase_Object` Actor))
  (`self.SetActorHiddenInGame` _asmap_base_object true)
  (`/Game/GameEditor/EditorPrograms/Editor/MyGameEditorPawn.CreateVirtualTips` (`/Game/GameEditor/EditorPrograms/Editor/FunctionLibrary/GetGamePawn.GetEditorPawn` 0) true)
  (`self.ManageOverlapedList` true)
  (`self.RestModelMaterial`))

(fn `Init`
  (locals (LocalModelRes :type "Resource Object Reference"))
  (set `self.ResId` (`VaRestJsonObject.GetStringField` (`self.ModelData`) "mxFileMD5"))
  (bind _returnvalue (`ModelFileComponent.GetPart` (`self.ModelFile`) 0))
  (`/Engine/EditorBlueprintResources/StandardMacros.IsValid` _returnvalue
    (:`Is Not Valid`
      (bind _returnvalue_2 (`ResourceMgr.Instance`))
      (if (not (`KismetStringLibrary.EqualEqual_StrStr` (`self.ResId`)))
        (bind _returnvalue_3 (`ResourceMgr.FindRes` _returnvalue_2 (`self.ResId`) false 0))
        (set `local.LocalModelRes` _returnvalue_3)
        (`/Engine/EditorBlueprintResources/StandardMacros.IsValid` (`local.LocalModelRes`)
          (:`Is Valid`
            (`self.UpdateModel` (`local.LocalModelRes`))))))))

(fn `ManageOverlapedList`
  (params (BeginOverlap :type Boolean) (actor :type "Actor Object Reference"))
  (locals (LocalActor :type "Actor Object Reference"))
  (bind _aioverlapedlist (`/Game/GameEditor/EditorPrograms/Editor/MyGameEditorPawn.AIOverlapedList` (`/Game/GameEditor/EditorPrograms/Editor/FunctionLibrary/GetGamePawn.GetEditorPawn` 0)))
  (bind _aioverlapedlist_2 (`/Game/GameEditor/EditorPrograms/Editor/MyGameEditorPawn.AIOverlapedList` (`/Game/GameEditor/EditorPrograms/Editor/FunctionLibrary/GetGamePawn.GetEditorPawn` 0)))
  (bind _output (`|GetArrayItem` _aioverlapedlist (`KismetArrayLibrary.Array_LastIndex` _aioverlapedlist)))
  (bind _output_2 (`|GetArrayItem` _aioverlapedlist_2 (`KismetArrayLibrary.Array_LastIndex` _aioverlapedlist_2)))
  (set `local.LocalActor` actor)
  (if BeginOverlap
    (if (> (`KismetArrayLibrary.Array_Length` (`/Game/GameEditor/EditorPrograms/Editor/MyGameEditorPawn.AIOverlapedList` (`/Game/GameEditor/EditorPrograms/Editor/FunctionLibrary/GetGamePawn.GetEditorPawn` 0))) 0)
      (`/Engine/EditorBlueprintResources/StandardMacros.IsValid` _output_2
        (:`Is Valid`
          (`self.SetVirtualMaterial` _output_2)
          (`KismetArrayLibrary.Array_AddUnique` (`/Game/GameEditor/EditorPrograms/Editor/MyGameEditorPawn.AIOverlapedList` (`/Game/GameEditor/EditorPrograms/Editor/FunctionLibrary/GetGamePawn.GetEditorPawn` 0)) self)))
      (else
        (`KismetArrayLibrary.Array_AddUnique` (`/Game/GameEditor/EditorPrograms/Editor/MyGameEditorPawn.AIOverlapedList` (`/Game/GameEditor/EditorPrograms/Editor/FunctionLibrary/GetGamePawn.GetEditorPawn` 0)) self)))
    (else
      (`KismetArrayLibrary.Array_RemoveItem` (`/Game/GameEditor/EditorPrograms/Editor/MyGameEditorPawn.AIOverlapedList` (`/Game/GameEditor/EditorPrograms/Editor/FunctionLibrary/GetGamePawn.GetEditorPawn` 0)) self)
      (if (> (`KismetArrayLibrary.Array_Length` (`/Game/GameEditor/EditorPrograms/Editor/MyGameEditorPawn.AIOverlapedList` (`/Game/GameEditor/EditorPrograms/Editor/FunctionLibrary/GetGamePawn.GetEditorPawn` 0))) 0)
        (`/Engine/EditorBlueprintResources/StandardMacros.IsValid` _output
          (:`Is Valid`
            (`self.RestModelMaterial` _output)
            (`/Game/GameEditor/EditorPrograms/Editor/MyGameEditorPawn.CreateVirtualTips` (`/Game/GameEditor/EditorPrograms/Editor/FunctionLibrary/GetGamePawn.GetEditorPawn` 0) true))
          (:`Is Not Valid`
            (bind _asmap_base_object (cast `/Game/GameEditor/EditorPrograms/MapObjectSystem/Base/MapBase_Object` (`local.LocalActor`) :!label _label))
            (`self.SetActorHiddenInGame` _asmap_base_object false)))
        (else
          (goto _label))))))

(fn `ResetAllVirtualObject`
  (locals (LocalVirtualObject :type "/Game/GameEditor/EditorPrograms/MapObjectSystem/Base/BP_VirtualObject Object Reference"))
  (bind _localvirtualobject (`local.LocalVirtualObject`))
  (for _array_element (`/Game/GameEditor/EditorPrograms/Editor/MyGameEditorPawn.VirtualObjectList` (`/Game/GameEditor/EditorPrograms/Editor/FunctionLibrary/GetGamePawn.GetEditorPawn` 0))
    (set `local.LocalVirtualObject` _array_element)
    (if (!= (`local.LocalVirtualObject`) self)
      (set `/Game/GameEditor/EditorPrograms/MapObjectSystem/Base/BP_VirtualObject.IsOverlap` false _localvirtualobject)
      (`self.SetVirtualMaterial` _localvirtualobject))))

(fn `RestModelMaterial`
  (locals (Local_Part :type "ModelPartComponent Object Reference") (Local_CurrentIndex :type Integer))
  (bind _output (`|GetArrayItem` (`self.OriginalMaterials`) (`local.Local_CurrentIndex`)))
  (set `self.IsOverlap` true)
  (bind _returnvalue (`ModelFileComponent.GetPart` (`self.ModelFile`) 0))
  (set `local.Local_Part` _returnvalue)
  (for _index (range (`ProceduralMeshComponent.GetNumSections` _returnvalue))
    (set `local.Local_CurrentIndex` _index)
    (if (`KismetArrayLibrary.Array_IsValidIndex` (`self.OriginalMaterials`))
      (`/Engine/EditorBlueprintResources/StandardMacros.IsValid` _output
        (:`Is Valid`
          (`PrimitiveComponent.SetMaterial` (`local.Local_Part`) (`local.Local_CurrentIndex`) _output))))))

(fn `SetAllVirtualMaterial`
  (locals (Local_Part :type "ModelPartComponent Object Reference"))
  (for _array_element (`/Game/GameEditor/EditorPrograms/Editor/MyGameEditorPawn.VirtualObjectList` (`/Game/GameEditor/EditorPrograms/Editor/FunctionLibrary/GetGamePawn.GetEditorPawn` 0))
    (bind _returnvalue (`ModelFileComponent.GetPart` (`/Game/GameEditor/EditorPrograms/MapObjectSystem/Base/BP_VirtualObject.ModelFile` _array_element) 0))
    (`/Engine/EditorBlueprintResources/StandardMacros.IsValid` _returnvalue
      (:`Is Valid`
        (set `local.Local_Part` _returnvalue)
        (for _index (range (`ProceduralMeshComponent.GetNumSections` (`local.Local_Part`)))
          (`PrimitiveComponent.SetMaterial` (`local.Local_Part`) _index "/Game/_Basic/Materials/Root/mesh.mesh"))))))

(fn `SetVirtualMaterial`
  (locals (Local_Part :type "ModelPartComponent Object Reference"))
  (set `self.IsOverlap` false)
  (bind _returnvalue (`ModelFileComponent.GetPart` (`self.ModelFile`) 0))
  (`/Engine/EditorBlueprintResources/StandardMacros.IsValid` _returnvalue
    (:`Is Valid`
      (set `local.Local_Part` _returnvalue)
      (for _index (range (`ProceduralMeshComponent.GetNumSections` (`local.Local_Part`)))
        (`PrimitiveComponent.SetMaterial` (`local.Local_Part`) _index "/Game/_Basic/Materials/Root/mesh_01.mesh_01")))))

(fn `UserConstructionScript`)