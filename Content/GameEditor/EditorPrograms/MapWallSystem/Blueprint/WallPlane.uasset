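; WallPlane is a map wall system actor in the game editor that builds a flat procedural mesh, apparently an area plane; its logic is commented as deprecated.
; On BeginPlay it raises every vertex in its list by a fixed Z offset.
; It then creates a procedural mesh section from those vertices and its triangle and normal arrays, and applies the area plane material.
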(event `self.ReceiveBeginPlay`
  (bind _verlist (`self.VerList`))
  ;[1 1 1] 弃用
  (for (_array_element _array_index) _verlist
    (`KismetArrayLibrary.Array_Set` _verlist _array_index (+ _array_element (0.0 0.0 281.0))))
  (`ProceduralMeshComponent.CreateMeshSection_LinearColor` :`self` (`self.Plane`) :`Vertices` (`self.VerList`) :`Triangles` (`self.Triangles`) :`Normals` (`self.NewVar_0`))
  (`PrimitiveComponent.SetMaterial` (`self.Plane`) 0 "/Game/GameEditor/EditorPrograms/MapWallSystem/Material/AreaPlaneMaterial.AreaPlaneMaterial"))

(fn `UserConstructionScript`)