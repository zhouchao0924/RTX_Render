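; TempPoint is a point marker actor for the map wall system in the game's editor, built from two flat cylinders.
; Every tick it rescales both cylinders from the player 2D camera's ortho width, so they track zoom, with Cylinder1 three times as wide as Cylinder.
; The SetHeidde event toggles hidden-in-game on the smaller Cylinder only.
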(event `SetHeidde`
  (params (Heidde :type Boolean))
  (`SceneComponent.SetHiddenInGame` (`self.Cylinder`) Heidde false))

(event `self.ReceiveTick`
  (params (DeltaSeconds :type "Float (single-precision)"))
  (bind _2dcamera (`/Game/GameEditor/EditorPrograms/MapWallSystem/Blueprint/FunctionLibrary/FunctionLibrary.GetPlayer2DCamera` 0))
  (`/Engine/EditorBlueprintResources/StandardMacros.IsValid` _2dcamera
    (:`Is Valid`
      (`SceneComponent.SetWorldScale3D` (`self.Cylinder`) (`KismetMathLibrary.MakeVector` (.x (`KismetMathLibrary.Conv_DoubleToVector` (/ (/ (`CameraComponent.OrthoWidth` _2dcamera) 1000.0) 15.0))) (.y (`KismetMathLibrary.Conv_DoubleToVector` (/ (/ (`CameraComponent.OrthoWidth` _2dcamera) 1000.0) 15.0))) 0.1))
      (`SceneComponent.SetWorldScale3D` (`self.Cylinder1`) (`KismetMathLibrary.MakeVector` (.x (`KismetMathLibrary.Conv_DoubleToVector` (/ (/ (`CameraComponent.OrthoWidth` (`/Game/GameEditor/EditorPrograms/MapWallSystem/Blueprint/FunctionLibrary/FunctionLibrary.GetPlayer2DCamera` 0)) 1000.0) 5.0))) (.y (`KismetMathLibrary.Conv_DoubleToVector` (/ (/ (`CameraComponent.OrthoWidth` (`/Game/GameEditor/EditorPrograms/MapWallSystem/Blueprint/FunctionLibrary/FunctionLibrary.GetPlayer2DCamera` 0)) 1000.0) 5.0))) 0.1)))))

(fn `UserConstructionScript`)