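; Placeable text note for the map wall editor, drawn as a NoteWidget in the viewport and removed when 2D mode turns off.
; On first creation it writes default settings into the game instance's ModelSavedConfig and spawns the widget.
; Selection reveals the Box and opens a NoteAttributes panel in the wall main widget.
; Tick fits the Box to the widget's desired size and applies the saved yaw.
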(event `self.ReceiveBeginPlay`
  (`parent.ReceiveBeginPlay`)
  (add `/Game/GameEditor/EditorPrograms/Editor/EditorGameInstance.2DMode` (`/Game/GameEditor/EditorPrograms/Editor/FunctionLibrary/GetEditorGameInstance.GetEditorGameInstance`) (delegate `CustomEvent`))
  (add `self.FirstCreated` (delegate `FirstCreated_事件_0`))
  (add `self.DR_SelectEvent` (delegate `DR_SelectEvent_Event`))
  (add `self.DR_UnSelectEvent` (delegate `DR_UnSelectEvent_Event`)))

(event `DR_SelectEvent_Event`
  (bind _returnvalue (`|CreateWidget` "/Game/GameEditor/EditorPrograms/MapWallSystem/Widget/Component/NoteAttributes.NoteAttributes_C" null self))
  (set `self.att` _returnvalue)
  (`/Game/GameEditor/EditorPrograms/MapWallSystem/Widget/W_WallDrawMainUI.AddAttributes` (`/Game/GameEditor/EditorPrograms/MapWallSystem/Blueprint/FunctionLibrary/FunctionLibrary.GetWallMainWidget`) _returnvalue)
  (`SceneComponent.SetHiddenInGame` (`self.Box`) false false))

(event `FirstCreated_事件_0`
  (bind _id (`self.ID`))
  (bind _ism2 (`self.ISM2`))
  (bind _modelsavedconfig (`/Game/GameEditor/EditorPrograms/Editor/EditorGameInstance.ModelSavedConfig` (`/Game/GameEditor/EditorPrograms/Editor/FunctionLibrary/GetEditorGameInstance.GetEditorGameInstance`)))
  (bind _item (`KismetArrayLibrary.Array_Get` _modelsavedconfig _id))
  (bind _structout (setmembers `/Game/GameEditor/EditorPrograms/Editor/Structure/SavedConfig/ModelSavedConfig_Other` :`StructRef` (`.Other_43_3A6DE2E141AA414E696319B252D72822` (break `/Game/GameEditor/EditorPrograms/Editor/Structure/SavedConfig/ModelSavedConfig` _item)) :`BoolSlot_01` false :`BoolSlot_02` _ism2 :`BoolSlot_03` _ism2 :`FloatSlot_01` 0.8 :`FloatSlot_02` 0.0 :`FloatSlot_03` 1.0 :`StringSlot_01` (`self.DefString`) :`ColorSlot_01` (struct :`R` 1.0 :`G` 1.0 :`B` 1.0 :`A` 1.0) :`ColorSlot_02` (struct :`R` 0.006 :`G` 0.006 :`B` 0.006 :`A` 1.0)))
  (bind _structout_2 (setmembers `/Game/GameEditor/EditorPrograms/Editor/Structure/SavedConfig/ModelSavedConfig` :`StructRef` _item :`Other` _structout))
  (`KismetArrayLibrary.Array_Set` _modelsavedconfig _id _structout_2 true)
  (bind _returnvalue (`|CreateWidget` "/Game/GameEditor/EditorPrograms/MapWallSystem/Widget/Component/NoteWidget.NoteWidget_C" null self :!label _label))
  (set `self.No` _returnvalue)
  (`UserWidget.AddToViewport` _returnvalue -1))

(event `DR_UnSelectEvent_Event`
  (`/Engine/EditorBlueprintResources/StandardMacros.IsValid` (stale `DR_SelectEvent_Event` _returnvalue)
    (:`Is Valid`
      (`Widget.RemoveFromParent` (stale `DR_SelectEvent_Event` _returnvalue)))
    (:`Is Not Valid`
      _))
  (`SceneComponent.SetHiddenInGame` (`self.Box`) true false))

(event `CustomEvent`
  (params (Is2D :type Boolean))
  (if Is2D
    (goto _label)
    (else
      (`/Engine/EditorBlueprintResources/StandardMacros.IsValid` (stale `FirstCreated_事件_0` _returnvalue)
        (:`Is Valid`
          (`Widget.RemoveFromParent` (stale `FirstCreated_事件_0` _returnvalue)))))))

(event `self.ReceiveTick`
  (params (DeltaSeconds :type "Float (single-precision)"))
  (bind _no (`self.No`))
  (bind (_x _y) (`KismetMathLibrary.BreakVector2D` (* (/ (`Widget.GetDesiredSize` (`/Game/GameEditor/EditorPrograms/MapWallSystem/Widget/Component/NoteWidget.Border_0` _no)) (`self.2DSize`)) 10.0)))
  (`parent.ReceiveTick` 0.0)
  (`/Engine/EditorBlueprintResources/StandardMacros.IsValid` _no
    (:`Is Valid`
      (`BoxComponent.SetBoxExtent` (`self.Box`) (`KismetMathLibrary.MakeVector` _y _x 1.0) true)
      (`self.K2_SetActorRotation` (`KismetMathLibrary.MakeRotator` 0.0 0.0 (`.FloatSlot_02_16_A2B259AC4F1A4B693CA307A93CA8FC1F` (break `/Game/GameEditor/EditorPrograms/Editor/Structure/SavedConfig/ModelSavedConfig_Other` (`.Other_43_3A6DE2E141AA414E696319B252D72822` (break `/Game/GameEditor/EditorPrograms/Editor/Structure/SavedConfig/ModelSavedConfig` (`KismetArrayLibrary.Array_Get` (`/Game/GameEditor/EditorPrograms/Editor/EditorGameInstance.ModelSavedConfig` (`/Game/GameEditor/EditorPrograms/Editor/FunctionLibrary/GetEditorGameInstance.GetEditorGameInstance`)) (`self.ID`)))))))))))

(event `self.ReceiveDestroyed`
  (bind _no (`self.No`))
  (bind _att (`self.att`))
  (`/Engine/EditorBlueprintResources/StandardMacros.IsValid` _no
    (:`Is Valid`
      (`Widget.RemoveFromParent` _no))
    (:`Is Not Valid`
      _))
  (`/Engine/EditorBlueprintResources/StandardMacros.IsValid` _att
    (:`Is Valid`
      (`Widget.RemoveFromParent` _att))))

(fn `UserConstructionScript`
  (`parent.UserConstructionScript`))